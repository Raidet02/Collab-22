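; Trigger volume that halts the player and sends them back to their starting position.
; On BeginPlay it caches player 0's capsule location and movement max acceleration.
; When a Player-tagged actor overlaps the box, it zeroes player 0's max acceleration, waits briefly, moves the capsule to the cached location without sweeping, then restores acceleration.
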(event OnComponentBeginOverlap(Box)
  (params (OverlappedComponent :type Primitive%20Component%20Object%20Reference) (OtherActor :type Actor%20Object%20Reference) (OtherComp :type Primitive%20Component%20Object%20Reference) (OtherBodyIndex :type Integer) (bFromSweep :type Boolean) (SweepResult :type Hit%20Result%20Structure%20%28by%20ref%29))
  (bind _returnvalue (Game|GetPlayerCharacter 0))
  (bind _charactermovement (Variables|/Script/Engine.Character|GetCharacterMovement _returnvalue))
  (if (Actor|ActorHasTag OtherActor "Player")
    (Variables|/Script/Engine.CharacterMovementComponent|SetMaxAcceleration _charactermovement 0.0)
    (Utilities|FlowControl|Delay 1.0)
    (Transformation|SetWorldLocation (Variables|/Script/Engine.Character|GetCapsuleComponent _returnvalue) (Variables|Default|GetInitialLoc) false false)
    (Variables|/Script/Engine.CharacterMovementComponent|SetMaxAcceleration _charactermovement (Variables|Default|GetInitialAcceleration))))

(event EventBeginPlay
  (bind _returnvalue (Game|GetPlayerCharacter 0))
  (Variables|Default|SetInitialLoc (Transformation|GetWorldLocation (Variables|/Script/Engine.Character|GetCapsuleComponent _returnvalue)))
  (Variables|Default|SetInitialAcceleration (Class|CharacterMovementComponent|GetMaxAcceleration (Variables|/Script/Engine.Character|GetCharacterMovement _returnvalue))))

(fn ConstructionScript)