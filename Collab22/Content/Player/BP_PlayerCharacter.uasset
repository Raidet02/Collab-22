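; Player character with cursor-based aiming, stepped camera zoom, timer-driven light/heavy combos with mixup, dodge and two weapon abilities.
; A spawned weapon Blueprint handles light attacks and abilities, while SetActionSettings toggles movement, action and damage flags.
; Stats live on the controller behind BPI_ControllerVars; damage passes through shield or health, with dispatchers broadcasting health, XP, death and cooldowns.
; Dodge launch is marked temporary, and several montage and win-screen paths are disconnected.
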(event Custom|HeavyAttackTimer
  ;[1 0 0 0.502 24] Heavy Attack Combo System
  ;;[0.15 0.15 0.15 0.5] When reached end of combo or player stopped attacking, resets attack increment and inflicts a cooldown before being able to restart the combo
  (Development|PrintString "Heavy Attack Finished" true true "(R=1.000000,G=1.000000,B=1.000000,A=1.000000)")
  (Variables|Combat|Internals|SetHeavyAttackIncrement 0)
  (bind _returnvalue (Utilities|Time|SetTimerbyEvent (delegate Custom|HeavyAttackCooldownReset) (Variables|Combat|Settings|HeavyAttack|GetHeavyAttackCooldown)))
  (Variables|Combat|Timers|HeavyAttack|SetHeavyAttackCooldownHandle _returnvalue))

(event Custom|OnTakeAnyDamage_Event
  (params (DamagedActor :type Actor%20Object%20Reference) (Damage :type Float%20%28single-precision%29) (DamageType :type Damage%20Type%20Object%20Reference) (InstigatedBy :type Controller%20Object%20Reference) (DamageCauser :type Actor%20Object%20Reference))
  ;[0.15 1 0.15 0.502 24] Health
  ;;[0.15 1 0.15 0.502] Inverses Damage Amount & Updates Health
  (if (Variables|Combat|Internals|ActionChecks|GetCanTakeDamage?)
    (CallFunction|UpdateHealth (* Damage -1.0))
    (Default|RecieveDamage (Variables|Default|GetAC_DamageNotification) "NewEnumerator1" (Transformation|GetWorldLocation (Variables|Collision|GetCapsuleComponent)) Damage false)))

(event Custom|AbilityCooldown
  ;[1 0 0 0.502 24] Player Ability System
  ;;[0.15 0.15 0.15 0.5] Sets ability ready to use
  (Variables|Combat|Internals|ActionChecks|SetCanUseAbility? true))

(event Custom|LightAttack
  ;[1 0 0 0.502 24] Light Attack Combo System
  (Math|Integer|IncrementInt (Variables|Combat|Internals|GetLightAttackIncrement)
    (:%20%20
      (bind _returnvalue (Utilities|Time|SetTimerbyEvent (EventDispatchers|CreateEvent :!event Custom|LightAttackTimer) 1.5))
      (Variables|Combat|Timers|LightAttack|SetLightAttackTimerHandle _returnvalue)
      (bind _returnvalue_2 (Utilities|Time|SetTimerbyEvent (EventDispatchers|CreateEvent :!event Custom|LightAttackWindow) (* 1.5 (Variables|Combat|Settings|LightAttack|GetLightAttackComboWindow))))
      (Variables|Combat|Timers|LightAttack|SetLightAttackWindowHandle _returnvalue_2))))

(event Custom|Win
  ;[0 0 0 0.5] TEMP Win/Lose
)

(event Custom|HeavyAttack
  ;[1 0 0 0.502 24] Heavy Attack Combo System
  (Animation|PlayAnimMontage (Utilities|Array|Get(acopy) (Variables|Combat|Animations|GetHeavyAttacks) (Variables|Combat|Internals|GetHeavyAttackIncrement)) 1.0 "None")
  (Math|Integer|IncrementInt (Variables|Combat|Internals|GetHeavyAttackIncrement)
    (:%20%20
      (Variables|Combat|Internals|ActionChecks|SetCanAttack? false)
      (bind _returnvalue (Utilities|Time|SetTimerbyEvent (EventDispatchers|CreateEvent :!event Custom|HeavyAttackTimer) 2.0))
      (Variables|Combat|Timers|HeavyAttack|SetHeavyAttackTimerHandle _returnvalue)
      (bind _returnvalue_2 (Utilities|Time|SetTimerbyEvent (EventDispatchers|CreateEvent :!event Custom|HeavyAttackWindow) (* 2.0 (Variables|Combat|Settings|HeavyAttack|GetHeavyAttackComboWindow))))
      (Variables|Combat|Timers|HeavyAttack|SetHeavyAttackWindowHandle _returnvalue_2))))

(event Custom|UpdateHealth
  (params (HealthAmount :type Float%20%28double-precision%29))
  (bind _returnvalue (Game|GetPlayerController 0))
  (bind _playerstats (Stats|GetCurrentPlayerStats))
  (bind _playerstats_2 (Stats|GetCurrentPlayerStats))
  (bind (_currenthealth _maxhealth) (Utilities|Struct|BreakF_PlayerStats _playerstats_2))
  ;[0.15 1 0.15 0.502 24] Health
  ;;[0.15 1 0.15 0.502] Updates Health Stat & Calls Event Dispatcher
  (if (Utilities|DoesObjectImplementInterface _returnvalue "/Game/Player/Interfaces/BPI_ControllerVars.BPI_ControllerVars_C")
    (if (Variables|Stats|GetHasShield?)
      ;;;[0.15 0.15 0.15 0.5] Uses Shield from staff ability if active
      (bind _output_get (Variables|Stats|SetShieldAmount (+ (Variables|Stats|GetShieldAmount) HealthAmount)))
      (if (<= _output_get 0.0)
        (Variables|Stats|SetHasShield? false))
      (else
        (Class|BPIControllerVars|UpdateCurrentHealth(Message) _returnvalue (Math|Float|Clamp(Float) (+ HealthAmount (.currenthealth _playerstats)) 0.0 (.maxhealth _playerstats)))))
    (Default|CallOnUpdateHealth _currenthealth _maxhealth)
    (if (<= (.CurrentHealth (Utilities|Struct|BreakF_PlayerStats (Stats|GetCurrentPlayerStats))) 0.0)
      (Default|CallOnDeath))))

(event Custom|HeavyAttackWindow
  ;[1 0 0 0.502 24] Heavy Attack Combo System
  ;;[0.15 0.15 0.15 0.5] The window for the player to input the next attack in the combo, defaulted to the last 20% of the animation
  (if (< (Variables|Combat|Internals|GetHeavyAttackIncrement) (Utilities|Array|Length (Variables|Combat|Animations|GetHeavyAttacks)))
    (Variables|Combat|Internals|ActionChecks|SetCanAttack? true)))

(event Custom|RevertDodgeSettings
  ;[1 0 0 0.502 24] Dodging
  (Utilities|SetActionSettings true true)
  (Development|PrintString "End Dodge"))

(event Custom|HeavyAttackCooldownReset
  ;[1 0 0 0.502 24] Heavy Attack Combo System
  ;;[0.15 0.15 0.15 0.5] When reached end of combo or player stopped attacking, resets attack increment and inflicts a cooldown before being able to restart the combo
  (Variables|Combat|Internals|ActionChecks|SetCanAttack? true)
  (Utilities|Time|ClearandInvalidateTimerbyHandle (Variables|Combat|Timers|HeavyAttack|GetHeavyAttackCooldownHandle)))

(event Custom|LightAttackTimer
  ;[1 0 0 0.502 24] Light Attack Combo System
  ;;[0.15 0.15 0.15 0.5] When reached end of combo or player stopped attacking, resets attack increment and inflicts a cooldown before being able to restart the combo
  (Development|PrintString "Light Attack Finished" true true "(R=1.000000,G=1.000000,B=1.000000,A=1.000000)")
  (Variables|Combat|Internals|SetLightAttackIncrement 0)
  (bind _returnvalue (Utilities|Time|SetTimerbyEvent (delegate Custom|Light%20Attack%20Cooldown%20Reset) (Variables|Combat|Settings|LightAttack|GetLightAttackCooldown)))
  (Variables|Combat|Timers|LightAttack|SetLightAttackCooldownHandle _returnvalue))

(event Custom|LightAttackWindow
  ;[1 0 0 0.502 24] Light Attack Combo System
  ;;[0.15 0.15 0.15 0.5] The window for the player to input the next attack in the combo, defaulted to the last 20% of the animation
  (if (< (Variables|Combat|Internals|GetLightAttackIncrement) (Utilities|Array|Length (Variables|Combat|Animations|GetLightAttacks)))
    (Variables|Combat|Internals|ActionChecks|SetCanAttack? true)))

(event Custom|Light%20Attack%20Cooldown%20Reset
  ;[1 0 0 0.502 24] Light Attack Combo System
  ;;[0.15 0.15 0.15 0.5] When reached end of combo or player stopped attacking, resets attack increment and inflicts a cooldown before being able to restart the combo
  (Variables|Combat|Internals|ActionChecks|SetCanAttack? true)
  (Utilities|Time|ClearandInvalidateTimerbyHandle (Variables|Combat|Timers|LightAttack|GetLightAttackCooldownHandle)))

(event Custom|AbilityFinish
  (bind _currentweapondata (Variables|Weapon|GetCurrentWeaponData))
  ;[1 0 0 0.502 24] Player Ability System
  ;;[0.15 0.15 0.15 0.5] When the ability has finished
  (Variables|Combat|Internals|ActionChecks|SetAbilityInUse? false)
  (Cosmetic|SetAimMarker)
  ;;;[0.15 0.15 0.15 0.5] Re-enable Bools
  (Utilities|SetActionSettings true false)
  ;;;[0.15 0.15 0.15 0.5] Cooldown Timer
  (Default|CallOnAbilityFinished (Utilities|Select :Index (Variables|Combat|Internals|GetAbilityInUse) :NewEnumerator0 (Variables|/Game/Player/Weapons/DataAssets/PDA_WeaponData_Parent.PDA_WeaponData_Parent_C|GetAbility1CooldownTime _currentweapondata) :NewEnumerator1 (Variables|/Game/Player/Weapons/DataAssets/PDA_WeaponData_Parent.PDA_WeaponData_Parent_C|GetAbility2CooldownTime _currentweapondata) :NewEnumerator2 0.0) (Variables|Combat|Internals|GetAbilityInUse))
  (Utilities|Time|SetTimerbyEvent (EventDispatchers|CreateEvent :!event Custom|AbilityCooldown) 3.0))

(event Input|EnhancedActionEvents|EnhancedInputActionIA_Move
  (params (ActionValue :type Vector%202D%20Structure) (ElapsedSeconds :type Float%20%28double-precision%29) (TriggeredSeconds :type Float%20%28double-precision%29) (InputAction :type Input%20Action%20Object%20Reference :default "/Game/Player/Input/InputActions/IA_Move.IA_Move"))
  ;[0.7969 0.5771 0 0.5 24] Input Actions
  ;;[0.3278 0.2346 0] Move
  (if (Variables|Combat|Internals|ActionChecks|GetCanMove?)
    (InputActions|Move (.x ActionValue) (.y ActionValue))))

(event Input|EnhancedActionEvents|EnhancedInputActionIA_Ability1
  (params (ActionValue :type Boolean) (ElapsedSeconds :type Float%20%28double-precision%29) (TriggeredSeconds :type Float%20%28double-precision%29) (InputAction :type Input%20Action%20Object%20Reference :default "/Game/Player/Input/InputActions/IA_Ability1.IA_Ability1"))
  (bind _currentweapondata (Variables|Weapon|GetCurrentWeaponData))
  (bind _currentweapondata_2 (Variables|Weapon|GetCurrentWeaponData))
  ;[1 0 0 0.502 24] Player Ability System
  ;;[0.15 0.15 0.15 0.5] Ability Input Action Events
  (:Started
    (Variables|Combat|Internals|SetAbilityInUse "NewEnumerator0")
    ;;;[0.15 0.15 0.15 0.5] Checks if there is an ongoing action, and if the ability is ready to be used
    (bind _actioninprogress_ (Utilities|CheckActioninProgress)
      (:%20%20
        (if (not _actioninprogress_)
          (if (Variables|Combat|Internals|ActionChecks|GetCanUseAbility?)
            ;;;[0.15 0.15 0.15 0.5] Sets booleans and selects the aim marker to set, as well as the animation montage to play depending on the ability
            (Variables|Combat|Internals|ActionChecks|SetCanUseAbility? false)
            (Variables|Combat|Internals|ActionChecks|SetAbilityInUse? true)
            (if (Utilities|Select :Index (Variables|Combat|Internals|GetAbilityInUse) :NewEnumerator0 (Variables|/Game/Player/Weapons/DataAssets/PDA_WeaponData_Parent.PDA_WeaponData_Parent_C|GetAbility1StopMovement? _currentweapondata) :NewEnumerator1 (Variables|/Game/Player/Weapons/DataAssets/PDA_WeaponData_Parent.PDA_WeaponData_Parent_C|GetAbility2StopMovement? _currentweapondata) :NewEnumerator2 false)
              (Utilities|SetActionSettings false false))
            ;;;[0.15 0.15 0.15 0.5] Ability Finish Timer
            (Cosmetic|SetAimMarker (Utilities|Select :Index (Variables|Combat|Internals|GetAbilityInUse) :NewEnumerator0 (Variables|/Game/Player/Weapons/DataAssets/PDA_WeaponData_Parent.PDA_WeaponData_Parent_C|GetAbility1AimMarker _currentweapondata_2) :NewEnumerator1 (Variables|/Game/Player/Weapons/DataAssets/PDA_WeaponData_Parent.PDA_WeaponData_Parent_C|GetAbility2AimMarker _currentweapondata_2) :NewEnumerator2 0))
            (Default|UseAbility (Variables|Weapon|GetCurrentWeaponBP) (Utilities|Select :Index (Variables|Combat|Internals|GetAbilityInUse) :NewEnumerator0 true :NewEnumerator1 false :NewEnumerator2 false))
            (Utilities|Time|SetTimerbyEvent (EventDispatchers|CreateEvent :!event Custom|AbilityFinish) 4.0)))))))

(event Input|EnhancedActionEvents|EnhancedInputActionIA_Aim
  (params (ActionValue :type Vector%202D%20Structure) (ElapsedSeconds :type Float%20%28double-precision%29) (TriggeredSeconds :type Float%20%28double-precision%29) (InputAction :type Input%20Action%20Object%20Reference :default "/Game/Player/Input/InputActions/IA_Aim.IA_Aim"))
  ;[0.7969 0.5771 0 0.5 24] Input Actions
  ;;[0.3278 0.2346 0] Look
  (InputActions|Aim false))

(event Input|EnhancedActionEvents|EnhancedInputActionIA_Dodge
  (params (ActionValue :type Boolean) (ElapsedSeconds :type Float%20%28double-precision%29) (TriggeredSeconds :type Float%20%28double-precision%29) (InputAction :type Input%20Action%20Object%20Reference :default "/Game/Player/Input/InputActions/IA_Dodge.IA_Dodge"))
  (bind _charactermovement (Variables|Character|GetCharacterMovement))
  (bind _velocity (Variables|/Script/Engine.MovementComponent|GetVelocity _charactermovement))
  ;[1 0 0 0.502 24] Dodging
  (:Started
    (if (Variables|Combat|Internals|ActionChecks|GetCanDodge?)
      (Utilities|SetActionSettings false true)
      (Development|PrintString "Start Dodge")
      ;;[0.15 0.15 0.15 0.5 24] ! TEMPORARY !                                                                                                                                                                         Dodge movement will be done in the anim montage via an animation notify state
      (Character|LaunchCharacter (* (select (> (Math|Vector|VectorLength _velocity) 0.0) (Math|Vector|Normalize _velocity) (Transformation|GetActorForwardVector)) (* (Variables|Combat|Settings|GetDodgeAmount) 1e+03)) false false)
      (Utilities|Time|SetTimerbyEvent (EventDispatchers|CreateEvent :!event Custom|RevertDodgeSettings) (Variables|Combat|Settings|GetDodgeCooldownTime))
      (Default|CallOnAbilityFinished (Variables|Combat|Settings|GetDodgeCooldownTime) "NewEnumerator2"))))

(event Input|EnhancedActionEvents|EnhancedInputActionIA_LightAttack
  (params (ActionValue :type Boolean) (ElapsedSeconds :type Float%20%28double-precision%29) (TriggeredSeconds :type Float%20%28double-precision%29) (InputAction :type Input%20Action%20Object%20Reference :default "/Game/Player/Input/InputActions/IA_LightAttack.IA_LightAttack"))
  ;[1 0 0 0.502 24] Light Attack Combo System
  ;;[0.15 0.15 0.15 0.5] Checks:                                                                                                                                                                                                                                                                                                                                                                         If player can attack?                                                                                                                                                                                                                                                                                                                                              If it's the first attack in the combo                                                                                                                                                                                                                                                                                                               If not first attack --> Clear full attack timer that ends the combo --> Play next attack in combo                                                                                                                                                                                        If first attack --> Play first attack in combo
  (if (Variables|Combat|Internals|ActionChecks|GetCanAttack?)
    (if (not (> (Variables|Combat|Internals|GetHeavyAttackIncrement) 0))
      (if (> (Variables|Combat|Internals|GetLightAttackIncrement) 0)
        (Utilities|Time|ClearandInvalidateTimerbyHandle (Variables|Combat|Timers|LightAttack|GetLightAttackTimerHandle))
        (Utilities|AttackDebug true (Variables|Combat|Internals|GetLightAttackIncrement) false :!label _label)
        (Variables|Combat|Internals|ActionChecks|SetCanAttack? false)
        (Utilities|Time|SetTimerbyEvent (EventDispatchers|CreateEvent :!event Custom|LightAttack) (/ 1.0 (.AttackSpeed (Utilities|Struct|BreakF_GameStats (Stats|GetCurrentGameStats)))))
        (Default|LightAttack (Variables|Weapon|GetCurrentWeaponBP) (Variables|Combat|Internals|GetLightAttackIncrement))
        (else
          (goto _label False))))))

(event Input|EnhancedActionEvents|EnhancedInputActionIA_HeavyAttack
  (params (ActionValue :type Boolean) (ElapsedSeconds :type Float%20%28double-precision%29) (TriggeredSeconds :type Float%20%28double-precision%29) (InputAction :type Input%20Action%20Object%20Reference :default "/Game/Player/Input/InputActions/IA_HeavyAttack.IA_HeavyAttack"))
  ;[1 0 0 0.502 24] Heavy Attack Combo System
  ;;[0.15 0.15 0.15 0.5] Checks:                                                                                                                                                                                                                                                                                                                    If player can attack?                                                                                                                                                                                                                                                                                                  If it's the first attack in the combo                                                                                                                                                                                                                                                                            If not first attack --> Clear full attack timer that ends the combo --> Play next attack in combo                                                                                                                                              If first attack --> Play first attack in combo
  (:Started
    (if (Variables|Combat|Internals|ActionChecks|GetCanAttack?)
      (if (> (Variables|Combat|Internals|GetLightAttackIncrement) 0)
        ;;;[0.15 0.15 0.15 0.5] Incorporates heavy attacks into light attacks
        (Combat|Internals|HeavyMixup)
        (elif (> (Variables|Combat|Internals|GetHeavyAttackIncrement) 0)
          (Utilities|Time|ClearandInvalidateTimerbyHandle (Variables|Combat|Timers|HeavyAttack|GetHeavyAttackTimerHandle))
          (else
            (goto _label False))))
      (Utilities|AttackDebug false (Variables|Combat|Internals|GetHeavyAttackIncrement) false :!label _label)
      (Variables|Combat|Internals|ActionChecks|SetCanAttack? false)
      (Utilities|Time|SetTimerbyEvent (EventDispatchers|CreateEvent :!event Custom|HeavyAttack) (/ 1.0 (.AttackSpeed (Utilities|Struct|BreakF_GameStats (Stats|GetCurrentGameStats))))))))

(event Input|EnhancedActionEvents|EnhancedInputActionIA_Ability2
  (params (ActionValue :type Boolean) (ElapsedSeconds :type Float%20%28double-precision%29) (TriggeredSeconds :type Float%20%28double-precision%29) (InputAction :type Input%20Action%20Object%20Reference :default "/Game/Player/Input/InputActions/IA_Ability2.IA_Ability2"))
  (bind _currentweapondata (Variables|Weapon|GetCurrentWeaponData))
  (bind _currentweapondata_2 (Variables|Weapon|GetCurrentWeaponData))
  ;[1 0 0 0.502 24] Player Ability System
  ;;[0.15 0.15 0.15 0.5] Ability Input Action Events
  (:Started
    (Variables|Combat|Internals|SetAbilityInUse "NewEnumerator1")
    ;;;[0.15 0.15 0.15 0.5] Checks if there is an ongoing action, and if the ability is ready to be used
    (bind _actioninprogress_ (Utilities|CheckActioninProgress)
      (:%20%20
        (if (not _actioninprogress_)
          (if (Variables|Combat|Internals|ActionChecks|GetCanUseAbility?)
            ;;;[0.15 0.15 0.15 0.5] Sets booleans and selects the aim marker to set, as well as the animation montage to play depending on the ability
            (Variables|Combat|Internals|ActionChecks|SetCanUseAbility? false)
            (Variables|Combat|Internals|ActionChecks|SetAbilityInUse? true)
            (if (Utilities|Select :Index (Variables|Combat|Internals|GetAbilityInUse) :NewEnumerator0 (Variables|/Game/Player/Weapons/DataAssets/PDA_WeaponData_Parent.PDA_WeaponData_Parent_C|GetAbility1StopMovement? _currentweapondata) :NewEnumerator1 (Variables|/Game/Player/Weapons/DataAssets/PDA_WeaponData_Parent.PDA_WeaponData_Parent_C|GetAbility2StopMovement? _currentweapondata) :NewEnumerator2 false)
              (Utilities|SetActionSettings false false))
            ;;;[0.15 0.15 0.15 0.5] Ability Finish Timer
            (Cosmetic|SetAimMarker (Utilities|Select :Index (Variables|Combat|Internals|GetAbilityInUse) :NewEnumerator0 (Variables|/Game/Player/Weapons/DataAssets/PDA_WeaponData_Parent.PDA_WeaponData_Parent_C|GetAbility1AimMarker _currentweapondata_2) :NewEnumerator1 (Variables|/Game/Player/Weapons/DataAssets/PDA_WeaponData_Parent.PDA_WeaponData_Parent_C|GetAbility2AimMarker _currentweapondata_2) :NewEnumerator2 0))
            (Default|UseAbility (Variables|Weapon|GetCurrentWeaponBP) (Utilities|Select :Index (Variables|Combat|Internals|GetAbilityInUse) :NewEnumerator0 true :NewEnumerator1 false :NewEnumerator2 false))
            (Utilities|Time|SetTimerbyEvent (EventDispatchers|CreateEvent :!event Custom|AbilityFinish) 4.0)))))))

(event Input|EnhancedActionEvents|EnhancedInputActionIA_CameraZoom
  (params (ActionValue :type Float%20%28double-precision%29) (ElapsedSeconds :type Float%20%28double-precision%29) (TriggeredSeconds :type Float%20%28double-precision%29) (InputAction :type Input%20Action%20Object%20Reference :default "/Game/Player/Input/InputActions/IA_CameraZoom.IA_CameraZoom"))
  ;[0 0 0 0.5] Camera Zoom
  (:Started
    (if (Variables|Default|GetHasZoomTimelineFinished?)
      (if (< ActionValue 0.0)
        (if (< (Variables|Default|GetZoomLevelIndex) 3)
          (Variables|Default|SetHasZoomTimelineFinished? false)
          (Math|Integer|IncrementInt (Variables|Default|GetZoomLevelIndex)
            (:%20%20
              (Variables|Default|SetRelative%20Location%20X (.x (Variables|/Script/Engine.SceneComponent|GetRelativeLocation (Variables|Default|GetCamera))))
              (bind _zoomout (Timeline|Timeline PlayFromStart)
                (:Update
                  (Transformation|SetRelativeLocation (Variables|Default|GetCamera) (Math|Vector|MakeVector (+ (Variables|Default|GetRelative%20Location%20X) _zoomout) 0.0 0.0) false false))
                (:Finished
                  (Variables|Default|SetHasZoomTimelineFinished? true))))))
        (elif (> (Variables|Default|GetZoomLevelIndex) 1)
          (Variables|Default|SetHasZoomTimelineFinished? false)
          (Math|Integer|DecrementInt (Variables|Default|GetZoomLevelIndex)
            (:%20%20
              (Variables|Default|SetRelative%20Location%20X (.x (Variables|/Script/Engine.SceneComponent|GetRelativeLocation (Variables|Default|GetCamera))))
              (bind _zoomin (Timeline|ChangeZoom PlayFromStart)
                (:Update
                  (Transformation|SetRelativeLocation (Variables|Default|GetCamera) (Math|Vector|MakeVector (+ (Variables|Default|GetRelative%20Location%20X) _zoomin) 0.0 0.0) false false))
                (:Finished
                  (Variables|Default|SetHasZoomTimelineFinished? true))))))))))

(event EventBeginPlay
  (bind _playerstats (Stats|GetCurrentPlayerStats))
  (bind _returnvalue (Game|GetPlayerController 0))
  (bind (_currenthealth _maxhealth) (Utilities|Struct|BreakF_PlayerStats _playerstats))
  ;[0.15 1 0.15 0.502] Health Events
  (EventDispatchers|AssignOnTakeAnyDamage (EventDispatchers|CreateEvent :!event Custom|OnTakeAnyDamage_Event))
  (Default|CallOnUpdateHealth _currenthealth _maxhealth)
  ;[0.15 1 0.15 0.502] Get Player Controller Ref
  (if (Utilities|DoesObjectImplementInterface _returnvalue "/Game/Player/Interfaces/BPI_ControllerVars.BPI_ControllerVars_C")
    (Variables|Default|SetPlayerControllerRef _returnvalue)))

(event EventGivePlayerXP
  (params (Amount :type Integer))
  ;[0.15 1 0.15 0.502 24] XP Events
  ;;[0.15 1 0.15 0.502] Give XP
  (Class|BPIControllerVars|UpdateCurrentXP(Message) (Variables|Default|GetPlayerControllerRef) Amount))

(event EventCallLevelUpdate
  (params (CurrentLevel :type Integer))
  ;[0.15 1 0.15 0.502 24] XP Events
  ;;[0.15 1 0.15 0.502] Link XP Dispatchers
  (Default|CallOnUpdateLevel CurrentLevel))

(event EventCallUpdateXP
  (params (CurrentXP :type Integer) (MaxXP :type Integer))
  ;[0.15 1 0.15 0.502 24] XP Events
  ;;[0.15 1 0.15 0.502] Link XP Dispatchers
  (Default|CallOnUpdateExperience CurrentXP MaxXP))

(event EventUpdateGameStats
  (params (NewStats :type F%20Game%20Stats%20Structure) (StatToUpdate :type E_UpgradeTypes%20Enum :default "NewEnumerator0"))
  ;[0 0 0 0.5] Update Non-Auto Stats
  (CallFunction|UpdateStats StatToUpdate))

(event EventGetGameModeRef
  (params (GameModeRef :type GM%20Player%20Test%20GM%20Object%20Reference))
  ;[0 0 0 0.5] TEMP Win/Lose
)

(event EventSetStartingWeapon
  (params (StartingWeapon :type PDA%20Weapon%20Data%20Parent%20Object%20Reference))
  ;[0.15 0.15 0.15 0.5] Set Char Weapon
  (bind _output_get (Variables|Weapon|SetCurrentWeaponData StartingWeapon))
  ;[0.15 0.15 0.15 0.5] Spawns Weapon in Hand
  (bind _returnvalue (Game|SpawnActorfromClass (Variables|/Game/Player/Weapons/DataAssets/PDA_WeaponData_Parent.PDA_WeaponData_Parent_C|GetWeaponBlueprint _output_get) (Transformation|GetRelativeTransform (Variables|Default|GetStaff)) "Undefined" "MultiplyWithRoot" 0 self 0))
  (bind _output_get_2 (Variables|Weapon|SetCurrentWeaponBP _returnvalue))
  (Transformation|AttachComponentToComponent _output_get_2 (Variables|Default|GetTEMP) "None" "KeepRelative" "KeepRelative" "KeepRelative" true))

(fn ConstructionScript
  ;[0.15 0.15 0.15 0.5] Sets the texture of the player's aim marker
  (bind _returnvalue (Rendering|Material|CreateDynamicMaterialInstance (Variables|Default|GetAimMarker) 0 0 "None" :!class /Script/Engine.PrimitiveComponent))
  (bind _output_get (Variables|Cosmetic|SetAimMarkerMaterial _returnvalue))
  (Rendering|Material|SetTextureParameterValue _output_get "None" 0))

(fn Move
  (params (X%20Axis :type Float%20%28double-precision%29) (Y%20Axis :type Float%20%28double-precision%29))
  (bind _returnvalue (Pawn|GetControlRotation :!class /Script/Engine.Pawn))
  ;[0.15 0.15 0.15 0.5] Initial Basic Movement
  (Pawn|Input|AddMovementInput (Math|Vector|GetRightVector (Math|Rotator|MakeRotator (.roll _returnvalue) 0.0 (.yaw _returnvalue))) X%20Axis false)
  (Pawn|Input|AddMovementInput (Math|Vector|GetForwardVector (Math|Rotator|MakeRotator 0.0 0.0 (.yaw (Pawn|GetControlRotation :!class /Script/Engine.Pawn)))) Y%20Axis false))

(fn Aim
  (params (DrawDebugLines? :type Boolean))
  (bind _lookingdirection (Variables|Default|GetLookingDirection))
  (bind _returnvalue (Math|Vector|GetForwardVector _lookingdirection))
  (bind _returnvalue_2 (Transformation|GetWorldLocation _lookingdirection))
  (if DrawDebugLines?
    (Rendering|Debug|DrawDebugLine _returnvalue_2 (+ (* _returnvalue 5e+02) _returnvalue_2) "(R=1.000000,G=0.192255,B=0.144003,A=1.000000)" 1.0 0.0))
  (Transformation|SetWorldRotation (Variables|Default|GetLookingDirection) (Math|Rotator|MakeRotator 0.0 0.0 (.yaw (Math|Rotator|FindLookatRotation (+ _returnvalue _returnvalue_2) (.Location (Collision|BreakHitResult (.HitResult (Game|Player|GetHitResultUnderCursorbyChannel (Game|GetPlayerController 0) "TraceTypeQuery1" true))))))) false false))

(fn GetCurrentPlayerStats
  (bind _returnvalue (Pawn|GetController))
  ;[0.15 0.15 0.15 0.5] Gets the player stats from the controller
  (if (Utilities|DoesObjectImplementInterface _returnvalue "/Game/Player/Interfaces/BPI_ControllerVars.BPI_ControllerVars_C")
    (bind _playerstats (Class|BPIControllerVars|GetPlayerStats(Message) _returnvalue))
    (return _playerstats)))

(fn HeavyMixup
  (Variables|Combat|Internals|SetHeavyAttackIncrement (- (Variables|Combat|Internals|GetLightAttackIncrement) 1))
  (Variables|Combat|Internals|SetLightAttackIncrement 0)
  (Utilities|Time|ClearandInvalidateTimerbyHandle (Variables|Combat|Timers|LightAttack|GetLightAttackTimerHandle))
  (return))

(fn SetAimMarker
  (params (Value :type Texture%20Object%20Reference))
  (Rendering|Material|SetTextureParameterValue (Variables|Cosmetic|GetAimMarkerMaterial) "None" Value))

(fn DoDamageCheck
  (params (Attacking? :type Boolean) (DamageTaken :type Float%20%28double-precision%29))
  (bind _chargamestats (Stats|GetCurrentGameStats))
  (bind (_attackdmg _attackspeed _defense _healthregen _healthmax _critrate _critdmg) (Utilities|Struct|BreakF_GameStats _chargamestats))
  (if Attacking?
    (LocalVariables|SetAttackDmg _attackdmg)
    (LocalVariables|SetDefense _defense)
    (LocalVariables|SetCritRate _critrate)
    (LocalVariables|SetCritDmg _critdmg)
    (if (<= (Math|Random|RandomIntegerinRange 1 100) (Math|Float|Truncate (LocalVariables|GetCritRate)))
      (return (* (LocalVariables|GetAttackDmg) (LocalVariables|GetCritDmg)))
      (else
        (return (LocalVariables|GetAttackDmg))))
    (else
      ;[0.15 0.15 0.15 0.5] If the player is being attacked
      (return (- DamageTaken (LocalVariables|GetDefense))))))

(fn ApplyDamage
  (params (ActorToDamage :type Actor%20Object%20Reference) (DamageType :type E_DamageTypes%20Enum :default "NewEnumerator0") (Attacking? :type Boolean) (DamageTaken :type Float%20%28double-precision%29))
  ;[0.15 0.15 0.15 0.5] Carries out Damage check and applies damage once or over time... Mainly to be used within anim montages
  (bind _damage (Combat|Damage|DoDamageCheck Attacking? DamageTaken))
  (bind _output_get (LocalVariables|SetDamageToApply _damage))
  (Default|CallOnAttackEnemy _output_get DamageType))

(fn GetCurrentGameStats
  (bind _returnvalue (Pawn|GetController))
  (if (Utilities|DoesObjectImplementInterface _returnvalue "/Game/Player/Interfaces/BPI_ControllerVars.BPI_ControllerVars_C")
    (bind _chargamestats (Class|BPIControllerVars|GetGameStats(Message) _returnvalue))
    (return _chargamestats)))

(fn StaffAttack
  (bind _returnvalue (Game|SpawnActorfromClass "/Game/Player/Weapons/BP_Staff_Projectile_base.BP_Staff_Projectile_base_C" (Math|Transform|MakeTransform (Transformation|GetWorldLocation (Variables|Default|GetLookingDirection)) "0, 0, 0" "1.000000,1.000000,1.000000") "Undefined" "MultiplyWithRoot" 0 0))
  (bind _damage (Combat|Damage|DoDamageCheck true 0.0))
  (Class|BPIStaffProjectile|GetInitalStats(Message) _returnvalue (Transformation|GetWorldRotation (Variables|Default|GetLookingDirection)) _damage))

(fn UpdateStats
  (params (Selection :type E_UpgradeTypes%20Enum :default "NewEnumerator0"))
  (switch Utilities|FlowControl|Switch|SwitchonE_UpgradeTypes Selection
    (:NewEnumerator4
      (Development|PrintString (Utilities|String|ToString(Float) (.MaxHealth (Utilities|Struct|BreakF_PlayerStats (Stats|GetCurrentPlayerStats))))))
    (:NewEnumerator7
      (Variables|/Script/Engine.CharacterMovementComponent|SetMaxWalkSpeed (Variables|Character|GetCharacterMovement) (.Speed (Utilities|Struct|BreakF_GameStats (Stats|GetCurrentGameStats)))))))

(fn SetShieldAmount
  (params (ShieldAmount :type Float%20%28double-precision%29))
  (Variables|Stats|SetShieldAmount ShieldAmount))

(fn GetShieldAmount
  (return (Variables|Stats|GetShieldAmount)))

(fn GetGameStats
  (return ""))

(fn GetPlayerHUD
  (return 0))

(fn GetplayerRef
  (return self))

(fn GetPlayerStats
  (return ""))