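; Base projectile for the player's staff, a fireball that damages what it overlaps.
; On BeginPlay it attaches a Niagara fireball to its collision sphere, with the effect's collision disabled.
; GetInitalStats receives damage, attack index and rotation, sets local-space velocity from the rotation's forward vector, and selects the effect by index, though all options currently match.
; Any sphere overlap applies the damage and destroys the projectile.
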(event OnComponentBeginOverlap(Sphere)
  (params (OverlappedComponent :type Primitive%20Component%20Object%20Reference) (OtherActor :type Actor%20Object%20Reference) (OtherComp :type Primitive%20Component%20Object%20Reference) (OtherBodyIndex :type Integer) (bFromSweep :type Boolean) (SweepResult :type Hit%20Result%20Structure%20%28by%20ref%29))
  (Game|Damage|ApplyDamage OtherActor (Variables|Default|GetDamage) 0 0)
  (Actor|DestroyActor))

(event EventGetInitalStats
  (params (Rotation :type Rotator :default "0, 0, 0") (Damage :type Float%20%28double-precision%29) (AtkIndex :type Integer))
  (Variables|Default|SetDamage Damage)
  (Variables|Default|SetAttackIndex AtkIndex)
  (Game|Components|ProjectileMovement|SetVelocityinLocalSpace (Variables|Default|GetProjectileMovement) (* (Math|Vector|GetForwardVector Rotation) 1e+03))
  (Class|NiagaraComponent|SetAsset (Variables|Default|GetParticalSystem) (Utilities|Select :Index (Variables|Default|GetAttackIndex) :Option%200 "/Game/Player/VFX/Staff/NS_Staff_FireBall_Base.NS_Staff_FireBall_Base" :Option%201 "/Game/Player/VFX/Staff/NS_Staff_FireBall_Base.NS_Staff_FireBall_Base" :Option%202 "/Game/Player/VFX/Staff/NS_Staff_FireBall_Base.NS_Staff_FireBall_Base") true))

(event EventBeginPlay
  (bind _returnvalue (Niagara|SpawnSystemAttached "/Game/Player/VFX/Staff/NS_Staff_FireBall_Base.NS_Staff_FireBall_Base" (Variables|Default|GetSphere) "None" "0, 0, 0" "0, 0, 0" "KeepRelativeOffset" false))
  (bind _output_get (Variables|Default|SetParticalSystem _returnvalue))
  (Collision|SetCollisionEnabled _output_get "NoCollision"))

(fn ConstructionScript)