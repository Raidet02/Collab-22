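; Base weapon Blueprint for the player, meant as the parent for specific weapons.
; On BeginPlay, Initialize applies the static mesh from WeaponData to the weapon mesh component if that data is valid.
; Light attack, heavy attack and two ability events are empty stubs, with UseAbility choosing between the abilities by a boolean.
; It also exposes a getter for the weapon data and a setter for the secondary damage type.
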(event Custom|Ability1)

(event Custom|Ability%202)

(event Custom|LightAttack
  (params (AttackIndex :type Integer)))

(event Custom|HeavyAttack
  (params (AttackIndex :type Integer)))

(event EventBeginPlay
  (CallFunction|Initialize))

(fn ConstructionScript)

(fn Initialize
  (bind _weapondata (Variables|Data|GetWeaponData))
  (Utilities|IsValid _weapondata
    (:Is%20Valid
      (Components|StaticMesh|SetStaticMesh (Variables|Default|GetWeaponMesh) (Variables|/Game/Player/Weapons/DataAssets/PDA_WeaponData_Parent.PDA_WeaponData_Parent_C|GetWeaponMesh _weapondata)))))

(fn GetWeaponData
  (return (Variables|Data|GetWeaponData)))

(fn UseAbility
  (params (UseAbility1? :type Boolean))
  (if UseAbility1?
    (CallFunction|Ability1)
    (else
      (CallFunction|Ability2))))

(fn SetSecondaryDmgType
  (params (SecondDamageType :type E_DamageTypes%20Enum :default "NewEnumerator0"))
  (Variables|Default|SetSecondDamageType SecondDamageType))