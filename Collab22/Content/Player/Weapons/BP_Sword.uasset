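; Player sword weapon with a light attack, a spin AoE and a knockback ability.
; Light attack damages enemies overlapping the blade, using the player's DoDamageCheck and a Niagara hit effect.
; Ability1 damages enemies in the AoE collision plus later entrants while enabled, tracking victims to avoid repeat hits.
; Ability2 fans line traces around the look direction and only collects detected enemies; no knockback is applied here.
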(event Custom|AoE_Overlap
  (params (OverlappedComponent :type Primitive%20Component%20Object%20Reference) (OtherActor :type Actor%20Object%20Reference) (OtherComp :type Primitive%20Component%20Object%20Reference) (OtherBodyIndex :type Integer) (bFromSweep :type Boolean) (SweepResult :type Hit%20Result%20Structure%20%28by%20ref%29))
  ;[0.15 0.15 0.15 0.5] Sword Spin AoE Attack
  ;;[0.15 0.15 0.15 0.5] Accounts for any enemies walking in area while spinning
  (if (Variables|Default|GetEnableAoECollision?)
    (Utilities|Array|Add (Variables|Default|GetOverlappedActors) OtherActor)
    (for _array_element (stale EventAbility1 _output_get)
      (if (> (Utilities|Array|Length (Variables|Default|GetAoEVictims)) 0)
        ;;[0.15 0.15 0.15 0.5] If already attacked enemies, add them to victims array, don't attack same enemy twice
        (if (not (Utilities|Array|ContainsItem (Variables|Default|GetAoEVictims) _array_element))
          (bind _damage (Default|DoDamageCheck (Variables|Default|GetPlayerChar) true 0.0 :!label _label))
          (Game|Damage|ApplyDamage _array_element _damage 0 0)
          (Utilities|IsValid _array_element
            (:Is%20Valid
              (Utilities|Array|Add (Variables|Default|GetAoEVictims) _array_element))))
        (else
          (goto _label))))))

(event EventBeginPlay
  (|CallParentFunction)
  (Collision|BindEventtoOnComponentBeginOverlap (Variables|Default|GetAoESlashCollision) (EventDispatchers|CreateEvent :!event Custom|AoE_Overlap)))

(event EventTick
  (params (DeltaSeconds :type Float%20%28single-precision%29)))

(event EventLightAttack
  (params (AttackIndex :type Integer))
  (bind _ns_hiteffect (Variables|Default|GetNS_HitEffect))
  (for _array_element (Collision|GetOverlappingActors (Variables|Default|GetSwordCollision) "/Game/Enemies/BP_Enemy_Parent.BP_Enemy_Parent_C" :!class /Script/Engine.PrimitiveComponent)
    (Transformation|AttachComponentToComponent _ns_hiteffect (Variables|/Script/Engine.Actor|GetRootComponent _array_element) "None" "KeepRelative" "KeepRelative" "KeepRelative" true)
    (bind _damage (Default|DoDamageCheck (Variables|Default|GetPlayerChar) true 0.0))
    (Game|Damage|ApplyDamage _array_element _damage 0 0)
    (Components|Activation|Activate _ns_hiteffect false)))

(event EventAbility1
  ;[0.15 0.15 0.15 0.5] Sword Spin AoE Attack
  (Variables|Default|SetEnableAoECollision? true)
  (bind _output_get (Variables|Default|SetOverlappedActors (Collision|GetOverlappingActors (Variables|Default|GetAoESlashCollision) "/Game/Enemies/BP_Enemy_Parent.BP_Enemy_Parent_C" :!class /Script/Engine.PrimitiveComponent)))
  (for _array_element _output_get
    (if (> (Utilities|Array|Length (Variables|Default|GetAoEVictims)) 0)
      ;;[0.15 0.15 0.15 0.5] If already attacked enemies, add them to victims array, don't attack same enemy twice
      (if (not (Utilities|Array|ContainsItem (Variables|Default|GetAoEVictims) _array_element))
        (bind _damage (Default|DoDamageCheck (Variables|Default|GetPlayerChar) true 0.0 :!label _label))
        (Game|Damage|ApplyDamage _array_element _damage 0 0)
        (Utilities|IsValid _array_element
          (:Is%20Valid
            (Utilities|Array|Add (Variables|Default|GetAoEVictims) _array_element))))
      (else
        (goto _label)))))

(event EventAbility2
  (bind _playerchar (Variables|Default|GetPlayerChar))
  (bind _knockbacktracediffs (Variables|Default|GetKnockbackTraceDiffs))
  (bind _lookingdirection (Variables|/Game/Player/BP_PlayerCharacter.BP_PlayerCharacter_C|GetLookingDirection _playerchar))
  (bind _returnvalue (Transformation|GetWorldLocation _lookingdirection))
  (for _index (range 0 (Variables|Default|GetKnockbackTraces))
    (if (< _index (Utilities|Array|Length _knockbacktracediffs))
      (bind _outhits (Class|KismetSystemLibrary|LineTraceMultiforObjects _returnvalue (Math|Vector|MakeVector (.X (Math|Vector|BreakVector (+ _returnvalue (Math|Vector|RotateVectorAroundAxis (* (Math|Vector|GetForwardVector _lookingdirection) (Variables|Default|GetKnockbackRange)) (Utilities|Array|Get(acopy) _knockbacktracediffs _index) "0.000000,0.000000,1.000000")))) (.Y (Math|Vector|BreakVector (+ _returnvalue (Math|Vector|RotateVectorAroundAxis (* (Math|Vector|GetForwardVector _lookingdirection) (Variables|Default|GetKnockbackRange)) (Utilities|Array|Get(acopy) _knockbacktracediffs _index) "0.000000,0.000000,1.000000")))) (.Z (Math|Vector|BreakVector _returnvalue))) (Utilities|Array|MakeArray "ObjectTypeQuery7") false 0 "ForDuration" true))
      (for _array_element _outhits
        (Utilities|Array|Add (Variables|Default|GetDetectedEnemies) 0)))))

(fn ConstructionScript
  (|CallParentFunction)
  (Class|NiagaraComponent|SetAsset (Variables|Default|GetNS_HitEffect) (Variables|/Game/Player/Weapons/DataAssets/PDA_WeaponData_Parent.PDA_WeaponData_Parent_C|GetAbility1Effect (Variables|Default|GetWeaponData)) true))