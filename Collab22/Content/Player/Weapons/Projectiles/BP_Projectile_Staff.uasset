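; Staff weapon fireball projectile that damages what it overlaps.
; On BeginPlay it attaches a Niagara fireball to its sphere, choosing the system by AttackIndex, though all options currently match, and starts a short timer, likely for self-destruction.
; Sphere overlap sends DamageTypeMap to the other actor through an ApplyDamageToEnemy message, then destroys the projectile.
; Older per-damage-type ApplyDamage calls remain as unused, deprecated nodes.
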(event OnComponentBeginOverlap(Sphere)
  (params (OverlappedComponent :type Primitive%20Component%20Object%20Reference) (OtherActor :type Actor%20Object%20Reference) (OtherComp :type Primitive%20Component%20Object%20Reference) (OtherBodyIndex :type Integer) (bFromSweep :type Boolean) (SweepResult :type Hit%20Result%20Structure%20%28by%20ref%29))
  ;[1 0 0 0.5] Apply Damage Types
  (Class|BPIEnemy|ApplyDamagetoEnemy(Message) OtherActor (Variables|Default|GetDamageTypeMap))
  (Actor|DestroyActor))

(event Custom|Destroy
  (Actor|DestroyActor))

(event EventBeginPlay
  ;[1 1 1 0.5] Attach VFX
  (bind _returnvalue (Niagara|SpawnSystemAttached "/Game/Player/VFX/Staff/NS_Staff_FireBall_Base.NS_Staff_FireBall_Base" (Variables|Default|GetSphere) "None" "0, 0, 0" "0, 0, 0" "KeepRelativeOffset" false))
  (bind _output_get (Variables|Default|SetParticalSystem _returnvalue))
  (Collision|SetCollisionEnabled _output_get "NoCollision")
  (Class|NiagaraComponent|SetAsset (Variables|Default|GetParticalSystem) (Utilities|Select :Index (Variables|Default|GetAttackIndex) :Option%200 "/Game/Player/VFX/Staff/NS_Staff_FireBall_Base.NS_Staff_FireBall_Base" :Option%201 "/Game/Player/VFX/Staff/NS_Staff_FireBall_Base.NS_Staff_FireBall_Base" :Option%202 "/Game/Player/VFX/Staff/NS_Staff_FireBall_Base.NS_Staff_FireBall_Base") true)
  (Utilities|Time|SetTimerbyEvent (EventDispatchers|CreateEvent :!event Custom|Destroy) 3.0))

(fn ConstructionScript)