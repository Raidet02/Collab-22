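; Game mode for a player test level that runs a timed round of enemy spawning.
; GetPlayerHUD starts the HUD countdown through the controller interface and hands the character a game mode reference.
; StartGame sets a matching world timer, configures mouse input, activates the player and tells the enemy manager to spawn.
; Other events pause or resume the timer, clear it on player death, or broadcast game completion when time runs out.
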(event Custom|TimerFinishEvent
  ;[0.15 0.15 0.15 0.5] Calls Game Complete & Returns to Base
  (Default|CallOnGameComplete))

(event EventStartGame
  (bind _returnvalue (Game|GetPlayerController 0))
  ;[0.15 0.15 0.15 0.5] Starts Game: World Timer, Activates player
  (bind _returnvalue_2 (Utilities|Time|SetTimerbyEvent (EventDispatchers|CreateEvent :!event Custom|TimerFinishEvent) 6e+02))
  (Variables|Timer|SetWorldTimerHandle _returnvalue_2)
  (if (Utilities|DoesObjectImplementInterface _returnvalue "/Game/Player/Interfaces/BPI_ControllerVars.BPI_ControllerVars_C")
    (Input|SetInputModeGameOnly _returnvalue false)
    (Variables|/Script/Engine.PlayerController|SetCurrentMouseCursor _returnvalue "Crosshairs")
    (Variables|/Script/Engine.PlayerController|SetbEnableClickEvents _returnvalue true)
    (Class|BPIControllerVars|SetActivatePlayer(Message) _returnvalue true)
    (bind _returnvalue_3 (Actor|GetActorOfClass "/Game/Enemies/BP_EnemyManager.BP_EnemyManager_C"))
    (Class|BPIEnemyManager|StartSpawn(Message) _returnvalue_3)))

(event EventToggleTimer
  (params (Paused? :type Boolean))
  (bind _worldtimerhandle (Variables|Timer|GetWorldTimerHandle))
  ;[0.15 0.15 0.15 0.5] Pause / Unpause Timer
  (if (Utilities|Time|IsValidTimerHandle (Variables|Timer|GetWorldTimerHandle))
    (if Paused?
      (Utilities|Time|PauseTimerbyHandle _worldtimerhandle)
      (else
        (Utilities|Time|UnpauseTimerbyHandle _worldtimerhandle)))
    (else
      (Development|PrintString "Timer Handle not Valid"))))

(event EventPlayerDead
  (bind _worldtimerhandle (Variables|Timer|GetWorldTimerHandle))
  ;[0.15 0.15 0.15 0.5] Delete Timer Event
  (if (Utilities|Time|IsValidTimerHandle _worldtimerhandle)
    (Utilities|Time|ClearandInvalidateTimerbyHandle _worldtimerhandle)))

(event EventGetPlayerHUD
  (bind _returnvalue (Game|GetPlayerController 0))
  (if (Utilities|DoesObjectImplementInterface _returnvalue "/Game/Player/Interfaces/BPI_ControllerVars.BPI_ControllerVars_C")
    (bind _output_get (Variables|Player|SetPlayerController _returnvalue))
    (bind _playerhud (Class|BPIControllerVars|GetPlayerHUD(Message) _output_get))
    (Default|StartGame _playerhud 10)
    (Class|BPIPlayer|GetGameModeRef(Message) (Game|GetPlayerCharacter 0) self)))

(fn ConstructionScript)