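; Main menu game mode that creates the title screen widget on BeginPlay, shows the mouse cursor and forces windowed fullscreen.
; After a timed delay, it enables skipping and runs a self-restarting timeline that fades the title text.
; The first pass uses its own opacity track, and later loops use the normal one.
; OpenMainMenu is an empty stub.
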(event Custom|Update%20Title%20Screen
  ;[1 1 1 0.5] Enable Skipping
  (Default|EnableSkipping (Variables|Default|GetTitle%20Screen))
  ;[1 1 1 0.5] Fades Title Screen Text In And Then Keep Keep Looping It
  (bind (_direction _1st_time_opacity _normal_opacity) (Timeline|Timeline PlayFromStart)
    (:Update
      (Default|UpdateTextOpacity (Variables|Default|GetTitle%20Screen) (Math|Float|SelectFloat _1st_time_opacity _normal_opacity (Variables|Default|Get1st%20Time?))))
    (:Finished
      (CallFunction|UpdateTitleScreen)
      (Variables|Default|Set1st%20Time? false))))

(event EventBeginPlay
  ;[1 1 1 0.5] Create Title Screen On Start Up
  (CallFunction|CreateTitleScreen)
  ;[1 1 1 0.5] Force Full Screen Mode For Startup
  (bind _returnvalue (Settings|GetGameUserSettings))
  (Class|GameUserSettings|SetFullscreenMode _returnvalue "WindowedFullscreen"))

(fn ConstructionScript)

(fn CreateTitleScreen
  (bind _returnvalue (Game|GetPlayerController 0))
  ;[1 1 1 0.5] Create Title Screen, Start It And Add It To Viewport
  (bind _returnvalue_2 (UserInterface|CreateWidget "/Game/UI/Widgets/Menus/WBP_TitleScreen.WBP_TitleScreen_C" _returnvalue))
  (bind _output_get (Variables|Default|SetTitle%20Screen _returnvalue_2))
  (Default|InitialiseWidget _output_get self)
  (UserInterface|Viewport|AddtoViewport _output_get 0)
  ;[1 1 1 0.5] Show Mouse Cursor, Set Title Screen To Active And Set Updates To Start After A Delay
  (Variables|/Script/Engine.PlayerController|SetbShowMouseCursor _returnvalue true)
  (Utilities|Time|SetTimerbyEvent (EventDispatchers|CreateEvent :!event Custom|Update%20Title%20Screen) (Variables|Default|GetWait%20Time)))

(fn OpenMainMenu)