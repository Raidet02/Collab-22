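; Base enemy Blueprint that fights the player, reports its death to an enemy manager and grants XP on EndPlay.
; InitEnemy stores the manager and scales health and damage by wave, then sets up the health bar.
; Incoming damage-type maps resolve into Defense-reduced damage or timed bleed/burn, stun and corrosion effects.
; Overlapping the attack radius damages the player, then slows the enemy during a timer-driven cooldown.
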(event OnComponentBeginOverlap(AttackDistanceRadius)
  (params (OverlappedComponent :type Primitive%20Component%20Object%20Reference) (OtherActor :type Actor%20Object%20Reference) (OtherComp :type Primitive%20Component%20Object%20Reference) (OtherBodyIndex :type Integer) (bFromSweep :type Boolean) (SweepResult :type Hit%20Result%20Structure%20%28by%20ref%29))
  ;[0 0 0 0.5] Attack + CD + Fall Back After Attack
  (if (Variables|Attack|GetCanAttack?)
    (Variables|Attack|SetCanAttack? false)
    (Variables|/Script/Engine.CharacterMovementComponent|SetMaxWalkSpeed (Variables|Character|GetCharacterMovement) 2e+02)
    (bind _returnvalue (Utilities|Time|SetTimerbyEvent (EventDispatchers|CreateEvent :!event Custom|ResetAttackCD) 1.0))
    (Variables|Attack|SetAttackTimer _returnvalue)
    (CallFunction|StartAttack)))

(event Custom|FollowPlayer
  (params (Destination :type Vector)))

(event Custom|FocusHealthBar)

(event Custom|StartAttack
  ;[0 0 0 0.5] Attack + CD + Fall Back After Attack
  (Game|Damage|ApplyDamage (Variables|Ref|GetPlayerRef) (Variables|Stats|GetDamageToDo) 0 0))

(event Custom|ResetAttackCD
  ;[0 0 0 0.5] Attack + CD + Fall Back After Attack
  (Variables|Attack|SetCanAttack? true)
  (Variables|/Script/Engine.CharacterMovementComponent|SetMaxWalkSpeed (Variables|Character|GetCharacterMovement) 6e+02))

(event Custom|DOT
  (bind _output_get (Variables|Stats|SetHealth (- (Variables|Stats|GetHealth) (Variables|UpgradeConditions|GetDOTDamage))))
  (if (<= _output_get 0.0)
    (Class|BPIEnemyManager|ChangeEnemySpawnedCount(Message) (Variables|Ref|GetEnemy%20Manager%20Ref) -1 self)
    (Actor|DestroyActor)
    (else
      (Default|CallOnHealthUpdated))))

(event Custom|ResetSpeed
  (Variables|/Script/Engine.CharacterMovementComponent|SetMaxWalkSpeed (Variables|Character|GetCharacterMovement) (Variables|Stats|GetSpeed)))

(event Custom|ResetDefence
  (Variables|Stats|SetDefense (Variables|UpgradeConditions|GetTempDefence)))

(event EventAttack)

(event EventInitEnemy
  (params (EnemyManagerRef :type Actor%20Object%20Reference) (WaveIndex :type Integer))
  (Variables|Ref|SetEnemy%20Manager%20Ref EnemyManagerRef)
  (CallFunction|SetStats WaveIndex))

(event EventApplyDamagetoEnemy
  (params (DamageTypeArray :type Map%20of%20E_DamageTypes%20Enums%20to%20Reals :default "NewEnumerator0"))
  (bind _damagedealt (CallFunction|CheckDamageTypes DamageTypeArray))
  (bind _output_get (Variables|Stats|SetHealth (- (Variables|Stats|GetHealth) (Math|Float|Clamp(Float) (- _damagedealt (Variables|Stats|GetDefense)) 0.0 _damagedealt))))
  (Default|RecieveDamage (Variables|Default|GetAC_DamageNotification) "NewEnumerator0" (Transformation|GetWorldLocation (Variables|Character|GetMesh)) (Math|Float|Clamp(Float) (- _damagedealt (Variables|Stats|GetDefense)) 0.0 _damagedealt) false)
  (if (<= _output_get 0.0)
    (Default|CallOnHealthUpdated)
    (Class|BPIEnemyManager|ChangeEnemySpawnedCount(Message) (Variables|Ref|GetEnemy%20Manager%20Ref) -1 self)
    (Actor|DestroyActor)
    (else
      (Default|CallOnHealthUpdated))))

(event EventGoto
  (params (Location :type Vector :default "0, 0, 0")))

(event EventEndPlay
  (params (EndPlayReason :type EEndPlayReason%20Enum :default "Destroyed"))
  (bind _returnvalue (Game|GetPlayerCharacter 0))
  (if (Utilities|DoesObjectImplementInterface _returnvalue "/Game/Player/Interfaces/BPI_XPReward.BPI_XPReward_C")
    (Class|BPIXPReward|GivePlayerXP(Message) _returnvalue (Variables|Stats|GetXPToGive))))

(event EventBeginPlay
  (Variables|Ref|SetPlayerRef (Game|GetPlayerCharacter 0)))

(event Game|Damage|EventAnyDamage
  (params (Damage :type Float%20%28single-precision%29) (DamageType :type Damage%20Type%20Object%20Reference) (InstigatedBy :type Controller%20Object%20Reference) (DamageCauser :type Actor%20Object%20Reference)))

(fn ConstructionScript)

(fn SetStats
  (params (WaveIndex :type Integer))
  (bind _output_get (LocalVariables|SetLocalWaveIndex (- WaveIndex 1)))
  (if (> _output_get 5)
    (LocalVariables|SetLocalWaveIndex 5))
  (Variables|Stats|SetDamageToDo (* (Utilities|Select :Index (LocalVariables|GetLocalWaveIndex) :Option%200 1.0 :Option%201 1.1 :Option%202 1.2 :Option%203 1.4 :Option%204 1.6) (Variables|Stats|GetDamageToDoBase)))
  (bind _output_get_2 (Variables|Stats|SetMaxHealth (Math|Conversions|ToFloat(Integer) (* (Utilities|Select :Index (LocalVariables|GetLocalWaveIndex) :Option%200 1.0 :Option%201 1.1 :Option%202 1.2 :Option%203 1.4 :Option%204 1.6) (Variables|Stats|GetMaxHealthBase)))))
  (Variables|Stats|SetHealth _output_get_2)
  ;[0 0 0 0.5] TEMP Health Bar
  (bind _aswbp_enemy_health_bar (Utilities|Casting|CastToWBP_EnemyHealthBar (UserInterface|GetWidget (Variables|Default|GetWidget))))
  (Default|Init _aswbp_enemy_health_bar self (Variables|Stats|GetMaxHealth)))

(fn CheckDamageTypes
  (params (DamageType :type Map%20of%20E_DamageTypes%20Enums%20to%20Reals :default "NewEnumerator0"))
  (bind (_keypin _valuepin) (Utilities|Map|ForEachLoop(Map) DamageType)
    (:then
      (bind _output_get (LocalVariables|SetDamage _valuepin))
      (if (> _output_get 0.0)
        (switch Utilities|FlowControl|Switch|SwitchonE_DamageTypes _keypin
          (:NewEnumerator0
            (return (LocalVariables|GetDamage)))
          (:NewEnumerator1
            (Variables|UpgradeConditions|SetDOTDamage (LocalVariables|GetDamage) :!label _label)
            (bind _returnvalue (Utilities|Time|SetTimerbyEvent (EventDispatchers|CreateEvent :!event Custom|DOT) 0.5 true))
            (Variables|UpgradeConditions|SetDOTTimer _returnvalue)
            (Variables|UpgradeConditions|SetTimesDOTApplied 0))
          (:NewEnumerator2
            (goto _label))
          (:NewEnumerator3
            (Variables|/Script/Engine.CharacterMovementComponent|SetMaxWalkSpeed (Variables|Character|GetCharacterMovement) 0.0)
            (Utilities|Time|SetTimerbyEvent (EventDispatchers|CreateEvent :!event Custom|ResetSpeed) 0.5))
          (:NewEnumerator4
            (bind _output_get_2 (Variables|UpgradeConditions|SetTempDefence (Variables|Stats|GetDefense)))
            (Variables|Stats|SetDefense (- _output_get_2 (LocalVariables|GetDamage)))
            (Utilities|Time|SetTimerbyEvent (EventDispatchers|CreateEvent :!event Custom|ResetSpeed) 0.5)))))))