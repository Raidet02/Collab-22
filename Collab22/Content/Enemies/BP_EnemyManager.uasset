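; Enemy manager that runs escalating enemy waves, spawning enemies at random reachable points around itself, intended to be off-screen.
; NextWave rearms a timer, grows the wave total, rebuilds the class pool by wave-index thresholds and spawns up to the total at once.
; Death reports lower the live count, starting the next wave early at zero.
; Random pure nodes re-evaluate, so returned locations may differ from those screen-tested; older spawning logic is disconnected.
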(event Custom|SpawnEnemies
  ;[0.15 0.15 0.15 0.5] Old Unoptimised Horror Code
)

(event Custom|WaveCheck
  ;[0.15 0.15 0.15 0.5] Old Unoptimised Horror Code
)

(event Custom|ResetOnce
  ;[0.15 0.15 0.15 0.5] Old Unoptimised Horror Code
)

(event Custom|StartSpawning_Event
  ;[0.15 0.15 0.15 0.5] Old Unoptimised Horror Code
)

(event Custom|SpawnEnemyLoop
  ;[0.15 0.15 0.15 0.5] New Updated Slightly More Optimised Still Horror Code
  (while (not (>= (Variables|EnemySpawn|GetEnemiesInWave) (Variables|EnemySpawn|GetTotalEnemiesInWave)))
    (Math|Integer|IncrementInt (Variables|EnemySpawn|GetEnemiesInWave)
      (:%20%20
        (CallFunction|Spawn)))))

(event Custom|Spawn
  ;[0.15 0.15 0.15 0.5] New Updated Slightly More Optimised Still Horror Code
  (bind (_isoffscreen _locationtospawn) (CallFunction|CalculateSpawnPosition (Variables|Ref|GetPlayerControllerRef)))
  (if _isoffscreen
    (bind _returnvalue (Game|SpawnActorfromClass (CallFunction|EnemytoSpawn) (Math|Transform|MakeTransform _locationtospawn "0, 0, 0" "1.000000,1.000000,1.000000") "AdjustIfPossibleButAlwaysSpawn" "MultiplyWithRoot" 0 0))
    (Default|CallOnEnemySpawned _returnvalue)
    (Class|BPIEnemy|InitEnemy(Message) _returnvalue self (Variables|Default|GetWave%20Index))))

(event Custom|NextWave
  (bind _availableenemypool (Variables|Default|GetAvailableEnemyPool))
  ;[0.15 0.15 0.15 0.5] New Updated Slightly More Optimised Still Horror Code
  ;;[0.15 0.15 0.15 0.5] Wave Initialiser
  (if (Utilities|Time|IsValidTimerHandle (Variables|Default|GetWaveTimer))
    (Utilities|Time|ClearandInvalidateTimerbyHandle (Variables|Default|GetWaveTimer)))
  (bind _returnvalue (Utilities|Time|SetTimerbyEvent (delegate Custom|NextWave) (Variables|Default|GetWaveTime)))
  (Variables|Default|SetWaveTimer _returnvalue)
  (Variables|EnemySpawn|SetTotalEnemiesInWave (+ (Math|Float|Truncate (* (Variables|EnemySpawn|GetTotalEnemiesInWave) 1.5)) (Variables|EnemySpawn|GetEnemiesInWave)))
  (Variables|Default|SetAmountToSpawn 0)
  (bind _result (Math|Integer|IncrementInt (Variables|Default|GetWave%20Index))
    (:%20%20
      (Utilities|Array|Clear _availableenemypool)
      (bind (_keypin _valuepin) (Utilities|Map|ForEachLoop(Map) (Variables|Default|GetEnemyClasses))
        (:then
          (if (>= _result _valuepin)
            (Utilities|Array|Add _availableenemypool _keypin)))
        (:CompletedPin
          (CallFunction|SpawnEnemyLoop))))))

(event EventBeginPlay
  ;[0.15 0.15 0.15 0.5] New Updated Slightly More Optimised Still Horror Code
  (Variables|Ref|SetPlayerControllerRef (Game|GetPlayerController 0)))

(event EventChangeEnemySpawnedCount
  (params (AmountToChange :type Integer) (EnemyKilledRef :type Actor%20Object%20Reference))
  ;[0.15 0.15 0.15 0.5] New Updated Slightly More Optimised Still Horror Code
  (Default|CallOnEnemyDied EnemyKilledRef)
  (if (<= (+ (Variables|EnemySpawn|GetEnemiesInWave) AmountToChange) 0)
    (Variables|EnemySpawn|SetEnemiesInWave 0)
    (CallFunction|NextWave)
    (else
      (Variables|EnemySpawn|SetEnemiesInWave (+ (Variables|EnemySpawn|GetEnemiesInWave) AmountToChange)))))

(event EventStartSpawn
  ;[0.15 0.15 0.15 0.5] New Updated Slightly More Optimised Still Horror Code
  (CallFunction|NextWave))

(fn ConstructionScript)

(fn CalculateSpawnPosition
  (params (PlayerController :type Player%20Controller%20Object%20Reference))
  (bind _returnvalue (Viewport|GetViewportSize))
  (bind _returnvalue_2 (Transformation|GetActorLocation))
  (bind _spawnradius (Variables|Default|GetSpawnRadius))
  (bind (_randomlocation _returnvalue_3) (AI|Navigation|GetRandomReachablePointinRadius _returnvalue_2 _spawnradius 0 0))
  (bind (_screenposition _returnvalue_4) (Class|GameplayStatics|ProjectWorldtoScreen PlayerController _randomlocation true))
  (while (not (Variables|Default|GetCanSpawnPoint))
    (if _returnvalue_3
      (if (not (Math|Boolean|ANDBoolean (and (>= (.x _screenposition) 0.0) (<= (.x _screenposition) (.x _returnvalue))) (and (>= (.y _screenposition) 0.0) (<= (.y _screenposition) (.y _returnvalue))) _returnvalue_4))
        (Variables|Default|SetCanSpawnPoint true))))
  (return true _randomlocation))

(fn EnemytoSpawn
  (return (.OutItem (Utilities|Array|Random (Variables|Default|GetAvailableEnemyPool)))))