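; Elite goblin enemy that roams near the player and acts as a buff aura for actors around it.
; A looping timer compares the player's position to the stored destination and, when they differ, sends the goblin via AIMoveTo to a random reachable point around the player.
; Its Sphere component sends a buff message to actors on begin overlap and a nerf message on end overlap, without filtering by type.
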(event OnComponentBeginOverlap(Sphere)
  (params (OverlappedComponent :type Primitive%20Component%20Object%20Reference) (OtherActor :type Actor%20Object%20Reference) (OtherComp :type Primitive%20Component%20Object%20Reference) (OtherBodyIndex :type Integer) (bFromSweep :type Boolean) (SweepResult :type Hit%20Result%20Structure%20%28by%20ref%29))
  (Class|BPIEnemy|BuffEnemy(Message) OtherActor))

(event OnComponentEndOverlap(Sphere)
  (params (OverlappedComponent :type Primitive%20Component%20Object%20Reference) (OtherActor :type Actor%20Object%20Reference) (OtherComp :type Primitive%20Component%20Object%20Reference) (OtherBodyIndex :type Integer))
  (Class|BPIEnemy|NerfEnemy(Message) OtherActor))

(event Custom|StartFollowListener
  (if (or (and (not (Variables|Default|GetisCurrentlyFollowing)) (Utilities|Operators|NotEqual(!=) (Variables|Default|GetCurrentPlayerLocation) (Transformation|GetActorLocation (Variables|Default|GetPlayerRef)) 1e+02)) (Utilities|Operators|NotEqual(!=) (Variables|Default|GetCurrentPlayerLocation) (Transformation|GetActorLocation (Variables|Default|GetPlayerRef)) 1e+02))
    (bind _output_get (Variables|Default|SetCurrentPlayerLocation (.RandomLocation (AI|Navigation|GetRandomReachablePointinRadius (Transformation|GetWorldLocation (Variables|/Script/Engine.Character|GetCapsuleComponent (Variables|Default|GetPlayerRef))) 1e+03 0 0))))
    (Variables|Default|SetisCurrentlyFollowing true)
    (AI|AIMoveTo self _output_get 0 5.0 false
      (:OnSuccess
        _)
      (:OnFail
        _))
    (Variables|Default|SetisCurrentlyFollowing false)))

(event EventBeginPlay
  (|CallParentFunction)
  (Utilities|Time|SetTimerbyEvent (delegate Custom|StartFollowListener) 0.7 true))

(fn ConstructionScript
  (|CallParentFunction))