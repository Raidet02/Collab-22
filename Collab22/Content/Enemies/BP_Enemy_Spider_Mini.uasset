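; BP_Enemy_Spider_Mini is a small spider enemy that alternates between roaming around the player and lunging at them.
; BeginPlay runs parent setup and SetStats, then starts a self-repeating AttackOrMove decision loop.
; Each move to a random reachable point near the player raises the next attack chance, up to guaranteed.
; An attack resets that chance, launches the spider toward the player, and re-decides after a short delay.
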(event Custom|MoveToNextLocation
  (AI|AIMoveTo self (.RandomLocation (AI|Navigation|GetRandomReachablePointinRadius (Transformation|GetWorldLocation (Variables|/Script/Engine.Character|GetCapsuleComponent (Variables|Default|GetPlayerRef))) 7.5e+02 0 0)) 0 1e+01 false
    (:OnSuccess
      (CallFunction|AttackorMove))
    (:OnFail
      (CallFunction|AttackorMove))))

(event Custom|AttackOrMove
  (if (<= (Math|Random|RandomIntegerinRange 1 100) (Utilities|Select :Index (Variables|Attack|GetChanceToAttackIndex) :Option%200 0 :Option%201 10 :Option%202 40 :Option%203 70 :Option%204 100))
    (Variables|Attack|SetChanceToAttackIndex 0)
    (CallFunction|InitiateAttack)
    (else
      (Math|Integer|IncrementInt (Variables|Attack|GetChanceToAttackIndex)
        (:%20%20
          (CallFunction|MovetoNextLocation))))))

(event Custom|InitiateAttack
  (Character|LaunchCharacter (* (Math|Vector|GetForwardVector (Math|Rotator|FindLookatRotation (Transformation|GetWorldLocation (Variables|Default|GetCapsuleComponent)) (Transformation|GetWorldLocation (Variables|/Script/Engine.Character|GetCapsuleComponent (Variables|Default|GetPlayerRef))))) 1e+03) false false)
  (Utilities|FlowControl|Delay 1.0)
  (CallFunction|AttackorMove))

(event EventBeginPlay
  (|CallParentFunction)
  (CallFunction|SetStats)
  (CallFunction|AttackorMove))

(fn ConstructionScript
  (|CallParentFunction))