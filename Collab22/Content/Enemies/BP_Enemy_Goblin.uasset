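; Goblin enemy Blueprint that chases the player by periodically re-targeting the player's position.
; A looping timer started on BeginPlay compares the player's location to the last stored one, with a distance tolerance.
; When the player has moved, it plays a 2D goblin noise, stores the new location and issues AIMoveTo there.
; The following flag clears on success or failure but never changes the condition's outcome.
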(event Custom|StartFollowListener
  (if (or (and (not (Variables|Default|GetisCurrentlyFollowing)) (Utilities|Operators|NotEqual(!=) (Variables|Default|GetCurrentPlayerLocation) (Transformation|GetActorLocation (Variables|Default|GetPlayerRef)) 1e+02)) (Utilities|Operators|NotEqual(!=) (Variables|Default|GetCurrentPlayerLocation) (Transformation|GetActorLocation (Variables|Default|GetPlayerRef)) 1e+02))
    (Audio|PlaySound2D "/Game/Audio/Assets/Enemy/S_GoblinNoise.S_GoblinNoise" 1.0 1.0 0.0 0 0)
    (bind _output_get (Variables|Default|SetCurrentPlayerLocation (Transformation|GetActorLocation (Variables|Default|GetPlayerRef))))
    (Variables|Default|SetisCurrentlyFollowing true)
    (AI|AIMoveTo self _output_get 0 5.0 false
      (:OnSuccess
        _)
      (:OnFail
        _))
    (Variables|Default|SetisCurrentlyFollowing false)))

(event EventBeginPlay
  (|CallParentFunction)
  (Utilities|Time|SetTimerbyEvent (delegate Custom|StartFollowListener) 0.7 true))

(fn ConstructionScript
  (|CallParentFunction))