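; Upgrade manager component that rolls upgrade options, tracks their levels for UI and applies chosen upgrades to player stats.
; Options come from a weighted random draw of three without replacement, from a pool whose weightings can be changed or removed.
; Stat upgrades multiply or add to the Game Instance's current values, while weapon choices message the assigned weapon upgrade object.
; Updated stats are then pushed to the player controller via interface.
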(event EventBeginPlay
  (bind _newparam (Class|BPIGameInstance|SetGameStats(Message) (Game|GetGameInstance)))
  (Variables|Default|SetCurrentStats _newparam))

(event EventSetWeaponUpgradeType
  (params (WeaponUpgrades :type AC%20Weapon%20Upgrades%20Base%20Object%20Reference))
  (Variables|Default|SetWeaponUpgrades WeaponUpgrades))

(event EventUpgradeStatLevel
  (params (UpgradeType :type E_UpgradeTypes%20Enum :default "NewEnumerator0") (ModifierValue :type Float%20%28double-precision%29))
  (bind _returnvalue (Math|Conversions|ToInteger(Byte) UpgradeType))
  (bind _upgradelevels (Variables|Default|GetUpgradeLevels))
  ;[0.7448 0.7448 0.7448 0.5] Increase stored level (For UI use)
  (Utilities|Array|SetArrayElem _upgradelevels _returnvalue (+ (Utilities|Array|Get(acopy) _upgradelevels _returnvalue) 1))
  (CallFunction|IncreaseStat UpgradeType ModifierValue))

(event EventGenerateUpgrades
  (CallFunction|RandomNewUpgrades))

(event EventRemovefromPool
  (params (UpgradeType :type E_UpgradeTypes%20Enum :default "NewEnumerator0"))
  (Utilities|Map|Remove (Variables|Default|GetBaseUpgradeWeightings) UpgradeType))

(event EventSetWeighting
  (params (UpgradeType :type E_UpgradeTypes%20Enum :default "NewEnumerator0") (Value :type Integer))
  (Utilities|Map|Add (Variables|Default|GetBaseUpgradeWeightings) UpgradeType Value))

(fn RandomNewUpgrade
  (params (PrevIndex :type Integer))
  ;[0.15 0.15 0.15 0.5] Loop until a new upgrade is found
  (while (LocalVariables|GetIsNotUnique)
    ;;[0.15 1 1 0.5] Generate a new int
    (LocalVariables|SetUpgradeInt (Utilities|Enum|ByteToEnumE_UpgradeTypes (Math|Conversions|ToByte(Integer) (Math|Random|RandomInteger 12))))
    ;;[1 0 0 0.5] Check Int is not in array
    (bind _index (Utilities|FlowControl|ForLoopwithBreak 0 PrevIndex :!label _label)
      (:LoopBody
        (bind _output_get (LocalVariables|SetInvalid (Utilities|Enum|Equal(Enum) (Utilities|Array|Get(acopy) (Variables|Default|GetUpgradeOptions) _index) (LocalVariables|GetUpgradeInt))))
        (if _output_get
          (goto _label Break)))
      (:Completed
        (if (not (LocalVariables|GetInvalid))
          (LocalVariables|SetIsNotUnique false)))))
  (return (LocalVariables|GetUpgradeInt)))

(fn SetStatsbyType
  (params (StatType :type E_StatTypes%20Enum :default "NewEnumerator0") (StatStruct :type F%20Game%20Stats%20Structure%20%28by%20ref%29) (Value :type Float%20%28double-precision%29))
  (LocalVariables|SetStruct StatStruct)
  (LocalVariables|SetNewValue Value)
  (switch Utilities|FlowControl|Switch|SwitchonE_StatTypes StatType
    (:NewEnumerator0
      (Utilities|Struct|SetmembersinF_GameStats (LocalVariables|GetStruct) (LocalVariables|GetNewValue)))
    (:NewEnumerator1
      (Utilities|Struct|SetmembersinF_GameStats (LocalVariables|GetStruct) (LocalVariables|GetNewValue)))
    (:NewEnumerator2
      (Utilities|Struct|SetmembersinF_GameStats (LocalVariables|GetStruct) (LocalVariables|GetNewValue)))
    (:NewEnumerator3
      (Utilities|Struct|SetmembersinF_GameStats (LocalVariables|GetStruct) (LocalVariables|GetNewValue)))
    (:NewEnumerator4
      (Utilities|Struct|SetmembersinF_GameStats (LocalVariables|GetStruct) (LocalVariables|GetNewValue)))
    (:NewEnumerator5
      (Utilities|Struct|SetmembersinF_GameStats (LocalVariables|GetStruct) (LocalVariables|GetNewValue)))
    (:NewEnumerator6
      (Utilities|Struct|SetmembersinF_GameStats (LocalVariables|GetStruct) (LocalVariables|GetNewValue)))
    (:NewEnumerator7
      (Utilities|Struct|SetmembersinF_GameStats (LocalVariables|GetStruct) (LocalVariables|GetNewValue)))
    (:NewEnumerator8
      (Utilities|Struct|SetmembersinF_GameStats (LocalVariables|GetStruct) (LocalVariables|GetNewValue))))
  (|SetBy-RefVar StatStruct (LocalVariables|GetStruct)))

(fn IncreaseStat
  (params (Type :type E_UpgradeTypes%20Enum :default "NewEnumerator0") (NewValue :type Float%20%28double-precision%29))
  ;[0.15 0.15 0.15 0.5] Apply Upgrade
  (LocalVariables|SetCurrentUpgrade Type)
  (LocalVariables|SetStatValue NewValue)
  (if (Utilities|DoesObjectImplementInterface (Components|GetOwner) "/Game/Player/Interfaces/BPI_ControllerVars.BPI_ControllerVars_C")
    _
    (else
      (Development|PrintText "Interface not implemented in owner" true true "(R=1.000000,G=0.000000,B=0.000000,A=1.000000)" 5.0)))
  (switch Utilities|FlowControl|Switch|SwitchonE_UpgradeTypes (LocalVariables|GetCurrentUpgrade)
    (:NewEnumerator0
      ;;[0.8 0.6 0 0.5] Multiplicative Stats
      (bind _gamestats (Class|BPIGameInstance|GetCurrentGameStats(Message) (Game|GetGameInstance) :!label _label))
      (CallFunction|SetStatsbyType (Utilities|Enum|ByteToEnumE_StatTypes (Math|Conversions|ToByte(Integer) (Math|Conversions|ToInteger(Byte) (LocalVariables|GetCurrentUpgrade)))) (Variables|Default|GetCurrentStats) (* (Utilities|Select :Index (Utilities|Enum|ByteToEnumE_StatTypes (Math|Conversions|ToByte(Integer) (Math|Conversions|ToInteger(Byte) (LocalVariables|GetCurrentUpgrade)))) :NewEnumerator0 (.attackdmg _gamestats) :NewEnumerator1 (.attackspeed _gamestats) :NewEnumerator2 0.0 :NewEnumerator3 0.0 :NewEnumerator4 (.healthmax _gamestats) :NewEnumerator5 (.critrate _gamestats) :NewEnumerator6 (.critdmg _gamestats) :NewEnumerator7 (.speed _gamestats) :NewEnumerator8 (.dashregen _gamestats)) (LocalVariables|GetStatValue))))
    (:NewEnumerator1
      (goto _label))
    (:NewEnumerator2
      ;;[0.15 0.6087 0.15 0.5] Additive Stats
      (bind _gamestats_2 (Class|BPIGameInstance|GetCurrentGameStats(Message) (Game|GetGameInstance) :!label _label_2))
      (CallFunction|SetStatsbyType (Utilities|Enum|ByteToEnumE_StatTypes (Math|Conversions|ToByte(Integer) (Math|Conversions|ToInteger(Byte) (LocalVariables|GetCurrentUpgrade)))) (Variables|Default|GetCurrentStats) (+ (Utilities|Select :Index (Utilities|Enum|ByteToEnumE_StatTypes (Math|Conversions|ToByte(Integer) (Math|Conversions|ToInteger(Byte) (LocalVariables|GetCurrentUpgrade)))) :NewEnumerator0 0.0 :NewEnumerator1 0.0 :NewEnumerator2 (.defense _gamestats_2) :NewEnumerator3 (.healthregen _gamestats_2) :NewEnumerator4 0.0 :NewEnumerator5 0.0 :NewEnumerator6 0.0 :NewEnumerator7 0.0 :NewEnumerator8 0.0) (LocalVariables|GetStatValue)))
      (Development|PrintString (Utilities|String|ToString(Float) (+ (Utilities|Select :Index (Utilities|Enum|ByteToEnumE_StatTypes (Math|Conversions|ToByte(Integer) (Math|Conversions|ToInteger(Byte) (LocalVariables|GetCurrentUpgrade)))) :NewEnumerator0 0.0 :NewEnumerator1 0.0 :NewEnumerator2 (.defense _gamestats_2) :NewEnumerator3 (.healthregen _gamestats_2) :NewEnumerator4 0.0 :NewEnumerator5 0.0 :NewEnumerator6 0.0 :NewEnumerator7 0.0 :NewEnumerator8 0.0) (LocalVariables|GetStatValue)))))
    (:NewEnumerator3
      (goto _label_2))
    (:NewEnumerator4
      (goto _label))
    (:NewEnumerator5
      (goto _label))
    (:NewEnumerator6
      (goto _label))
    (:NewEnumerator7
      (goto _label))
    (:NewEnumerator8
      (goto _label))
    (:NewEnumerator15
      ;;[1 1 1 0.5] WeaponUpgrades
      (Class|BPIWeaponUpgrade|Upgrade1(Message) (Variables|Default|GetWeaponUpgrades) 3.0))
    (:NewEnumerator16
      (Class|BPIWeaponUpgrade|Upgrade2(Message) (Variables|Default|GetWeaponUpgrades) 0.2))
    (:NewEnumerator17
      (Class|BPIWeaponUpgrade|Upgrade3(Message) (Variables|Default|GetWeaponUpgrades) 1.0)))
  ;;[1 0 0 0.5] Update Player Stats (BPI_ControllerVars)
  (Class|BPIControllerVars|UpdateGameStats(Message) (Game|GetPlayerController 0) (Variables|Default|GetCurrentStats) (LocalVariables|GetCurrentUpgrade)))

(fn RandomNewUpgrades
  ;[0.15 1 1 0.502] Find total weighting for random number generation
  (LocalVariables|SetUpgradeWeightings (Variables|Default|GetBaseUpgradeWeightings))
  (bind _valuepin (Utilities|Map|ForEachLoop(Map) (LocalVariables|GetUpgradeWeightings))
    (:then
      (LocalVariables|SetTotalWeight (+ _valuepin (LocalVariables|GetTotalWeight))))
    (:CompletedPin
      (for _index (range 0 2)
        ;[1 1 1 0.5] Generate a random upgrade type from weighting
        ;;[0.15 1 1 0.502] Generate a new int
        (LocalVariables|SetCurrentInt (Math|Random|RandomInteger (LocalVariables|GetTotalWeight)))
        (bind (_keypin _valuepin_2) (Utilities|Map|ForEachLoop(Map) (LocalVariables|GetUpgradeWeightings) :!label _label)
          (:then
            (if (< (LocalVariables|GetCurrentInt) _valuepin_2)
              (Utilities|Array|SetArrayElem (Variables|Default|GetUpgradeOptions) _index _keypin)
              (Utilities|Map|Remove (LocalVariables|GetUpgradeWeightings) _keypin)
              (LocalVariables|SetTotalWeight (- (LocalVariables|GetTotalWeight) _valuepin_2))
              (goto _label BreakPin)
              (else
                (LocalVariables|SetCurrentInt (- (LocalVariables|GetCurrentInt) _valuepin_2))))))))))

(fn GetCurrentGameStats
  (return (Variables|Default|GetCurrentStats)))

(fn GetStatLevel
  (params (UpgradeType :type E_UpgradeTypes%20Enum :default "NewEnumerator0"))
  (return (Utilities|Array|Get(acopy) (Variables|Default|GetUpgradeLevels) (Math|Conversions|ToInteger(Byte) UpgradeType))))

(fn GetUpgradeOption
  (params (Index :type Integer))
  (return (Utilities|Array|Get(acopy) (Variables|Default|GetUpgradeOptions) Index)))