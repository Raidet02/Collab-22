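; BP_Stats holds gold, stat modifiers and upgrade costs for purchasable upgrades to Attack, Defence, Attack Speed and Health Regen.
; MetaUpgradeEvent calls UpgradeStat, which checks that gold covers the chosen stat's cost, deducts it and returns whether the purchase succeeded.
; Each purchase compounds that stat's modifier and price by fixed multipliers, with cost rising faster.
; Getters expose modifiers, current stats and truncated gold.
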(event Custom|MetaUpgradeEvent
  (params (StatType :type E_StatType%20Enum :default "NewEnumerator0"))
  (CallFunction|UpgradeStat StatType))

(fn UpgradeStat
  (params (Stat :type E_StatType%20Enum :default "NewEnumerator0"))
  (LocalVariables|SetCurrentStat Stat)
  (bind _output_get (LocalVariables|SetValid (>= (- (Variables|Default|GetGold) (Utilities|Select :Index (LocalVariables|GetCurrentStat) :NewEnumerator0 (.attack (Variables|Default|GetCostOfStats)) :NewEnumerator1 (.defence (Variables|Default|GetCostOfStats)) :NewEnumerator2 (.attackspeed (Variables|Default|GetCostOfStats)) :NewEnumerator3 (.healthregen (Variables|Default|GetCostOfStats)))) 0.0)))
  (if _output_get
    (Variables|Default|SetGold (- (Variables|Default|GetGold) (Utilities|Select :Index (LocalVariables|GetCurrentStat) :NewEnumerator0 (.attack (Variables|Default|GetCostOfStats)) :NewEnumerator1 (.defence (Variables|Default|GetCostOfStats)) :NewEnumerator2 (.attackspeed (Variables|Default|GetCostOfStats)) :NewEnumerator3 (.healthregen (Variables|Default|GetCostOfStats)))))
    ;[0.15 0.15 0.15 0.5 33] Updating stats and upgrade costs
    (switch Utilities|FlowControl|Switch|SwitchonE_StatType (LocalVariables|GetCurrentStat)
      (:NewEnumerator0
        (Variables|Default|SetModStats (Utilities|Struct|MakeF_GameStats (* (.attack (Variables|Default|GetModStats)) 1.1) (.defence (Variables|Default|GetModStats)) (.attackspeed (Variables|Default|GetModStats)) (.healthregen (Variables|Default|GetModStats))))
        (Variables|Default|SetCostOfStats (Utilities|Struct|MakeF_GameStats (* (.attack (Variables|Default|GetCostOfStats)) 1.5) (.defence (Variables|Default|GetCostOfStats)) (.attackspeed (Variables|Default|GetCostOfStats)) (.healthregen (Variables|Default|GetCostOfStats)))))
      (:NewEnumerator1
        (Variables|Default|SetModStats (Utilities|Struct|MakeF_GameStats (.attack (Variables|Default|GetModStats)) (* (.defence (Variables|Default|GetModStats)) 1.1) (.attackspeed (Variables|Default|GetModStats)) (.healthregen (Variables|Default|GetModStats))))
        (Variables|Default|SetCostOfStats (Utilities|Struct|MakeF_GameStats (.attack (Variables|Default|GetCostOfStats)) (* (.defence (Variables|Default|GetCostOfStats)) 1.5) (.attackspeed (Variables|Default|GetCostOfStats)) (.healthregen (Variables|Default|GetCostOfStats)))))
      (:NewEnumerator2
        (Variables|Default|SetModStats (Utilities|Struct|MakeF_GameStats (.attack (Variables|Default|GetModStats)) (.defence (Variables|Default|GetModStats)) (* (.attackspeed (Variables|Default|GetModStats)) 1.1) (.healthregen (Variables|Default|GetModStats))))
        (Variables|Default|SetCostOfStats (Utilities|Struct|MakeF_GameStats (.attack (Variables|Default|GetCostOfStats)) (.defence (Variables|Default|GetCostOfStats)) (* (.attackspeed (Variables|Default|GetCostOfStats)) 1.5) (.healthregen (Variables|Default|GetCostOfStats)))))
      (:NewEnumerator3
        (Variables|Default|SetModStats (Utilities|Struct|MakeF_GameStats (.attack (Variables|Default|GetModStats)) (.defence (Variables|Default|GetModStats)) (.attackspeed (Variables|Default|GetModStats)) (* (.healthregen (Variables|Default|GetModStats)) 1.1)))
        (Variables|Default|SetCostOfStats (Utilities|Struct|MakeF_GameStats (.attack (Variables|Default|GetCostOfStats)) (.defence (Variables|Default|GetCostOfStats)) (.attackspeed (Variables|Default|GetCostOfStats)) (* (.healthregen (Variables|Default|GetCostOfStats)) 1.5))))))
  (return (LocalVariables|GetValid)))

(fn GetModifierStats
  (return (Variables|Default|GetModStats)))

(fn GetCurrentStats
  (return (Variables|Default|GetCurrentStats)))

(fn GetGold
  (return (Math|Float|Truncate (Variables|Default|GetGold))))