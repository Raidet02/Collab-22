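; Bow projectile that damages actors it overlaps, with Arrow Storm and pierce effects.
; Each collider overlap applies damage, then rolls against StormChance to possibly spawn a BP_ArrowStorm at the projectile's transform.
; PierceCount drops with each overlap, and the projectile destroys itself on an overlap once none remain.
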(event OnComponentBeginOverlap(Collider)
  (params (OverlappedComponent :type Primitive%20Component%20Object%20Reference) (OtherActor :type Actor%20Object%20Reference) (OtherComp :type Primitive%20Component%20Object%20Reference) (OtherBodyIndex :type Integer) (bFromSweep :type Boolean) (SweepResult :type Hit%20Result%20Structure%20%28by%20ref%29))
  (Game|Damage|ApplyDamage OtherActor (Variables|Default|GetDamage) 0 0)
  ;[0.15 0.15 0.15 0.5] Arrow Storm
  (if (>= (Math|Random|RandomIntegerinRange 0 100) (Variables|Default|GetStormChance))
    _
    (else
      (Game|SpawnActorfromClass "/Game/Upgrades/UpgradeAbilities/BP_ArrowStorm.BP_ArrowStorm_C" (Transformation|GetActorTransform self) "Undefined" "MultiplyWithRoot" 0 0)))
  ;[1 0 0 0.5] Pierce
  (if (<= (Variables|Default|GetPierceCount) 0)
    (Actor|DestroyActor)
    (else
      (Variables|Default|SetPierceCount (- (Variables|Default|GetPierceCount) 1)))))

(fn ConstructionScript)