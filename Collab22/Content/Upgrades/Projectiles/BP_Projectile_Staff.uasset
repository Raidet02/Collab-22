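; BP_Projectile_Staff is the staff's projectile, shown as a Niagara fireball that deals several damage types on overlap.
; BeginPlay attaches the effect to the Sphere, disables its collision and re-sets its asset through a Select whose options are all the same base fireball.
; Sphere overlap applies corrosion, base, burn and stun damage to the other actor, passing stun duration as the damage amount, then destroys the projectile.
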(event OnComponentBeginOverlap(Sphere)
  (params (OverlappedComponent :type Primitive%20Component%20Object%20Reference) (OtherActor :type Actor%20Object%20Reference) (OtherComp :type Primitive%20Component%20Object%20Reference) (OtherBodyIndex :type Integer) (bFromSweep :type Boolean) (SweepResult :type Hit%20Result%20Structure%20%28by%20ref%29))
  (Game|Damage|ApplyDamage OtherActor (Math|Conversions|ToFloat(Integer) (Variables|Upgrades|GetCorrosionDamage)) 0 0 "/Game/Upgrades/UpgradeAbilities/DamageType_Corrosion.DamageType_Corrosion_C")
  (Game|Damage|ApplyDamage OtherActor (Variables|Default|GetDamage) 0 0)
  (Game|Damage|ApplyDamage OtherActor (Math|Conversions|ToFloat(Integer) (Variables|Upgrades|GetBurnDamage)) 0 0 "/Game/Upgrades/UpgradeAbilities/DamageType_Burn.DamageType_Burn_C")
  (Game|Damage|ApplyDamage OtherActor (Variables|Upgrades|GetStunDuration) 0 0 "/Game/Upgrades/UpgradeAbilities/DamageType_Stun.DamageType_Stun_C")
  (Actor|DestroyActor))

(event EventBeginPlay
  (bind _returnvalue (Niagara|SpawnSystemAttached "/Game/Player/VFX/Staff/NS_Staff_FireBall_Base.NS_Staff_FireBall_Base" (Variables|Default|GetSphere) "None" "0, 0, 0" "0, 0, 0" "KeepRelativeOffset" false))
  (bind _output_get (Variables|Default|SetParticalSystem _returnvalue))
  (Collision|SetCollisionEnabled _output_get "NoCollision")
  (Class|NiagaraComponent|SetAsset (Variables|Default|GetParticalSystem) (Utilities|Select :Index 0 :Option%200 "/Game/Player/VFX/Staff/NS_Staff_FireBall_Base.NS_Staff_FireBall_Base" :Option%201 "/Game/Player/VFX/Staff/NS_Staff_FireBall_Base.NS_Staff_FireBall_Base" :Option%202 "/Game/Player/VFX/Staff/NS_Staff_FireBall_Base.NS_Staff_FireBall_Base") true))

(fn ConstructionScript)