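; Test actor for a multishot upgrade that automatically fires fans of arrow projectiles toward the mouse cursor.
; On BeginPlay, looping timers turn an Arrow component toward the cursor hit point and call FireMultishot.
; FireMultishot divides a 90-degree arc by ProjCount and spawns BP_Test_Projectile_Arrow actors at even yaw steps centered on the arrow's heading.
; An unconnected single-shot spawn remains in the event graph.
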(event Custom|RotateToMouse
  (bind _returnvalue (Game|GetPlayerController 0))
  (bind _returnvalue_2 (Transformation|GetActorLocation))
  (bind _hitresult (Game|Player|GetHitResultUnderCursorbyChannel _returnvalue "TraceTypeQuery1" true))
  (bind _returnvalue_3 (Math|Rotator|FindLookatRotation _returnvalue_2 (.location _hitresult)))
  ;[0.15 0.15 0.15 0.5] Arrow Rotation and Fire Interval (Ignore)
  (Transformation|SetWorldTransform (Variables|Default|GetArrow) (Math|Transform|MakeTransform _returnvalue_2 (Math|Rotator|MakeRotator (.roll _returnvalue_3) 0.0 (.yaw _returnvalue_3)) "1.000000,1.000000,1.000000") false false))

(event Custom|FireProj
  ;[0.15 0.15 0.15 0.5] Arrow Rotation and Fire Interval (Ignore)
  (CallFunction|FireMultishot))

(event EventBeginPlay
  ;[0.15 0.15 0.15 0.5] Arrow Rotation and Fire Interval (Ignore)
  (Utilities|Time|SetTimerbyEvent (delegate Custom|RotateToMouse) 0.05 true)
  (Utilities|Time|SetTimerbyEvent (delegate Custom|FireProj) 0.6 true))

(fn ConstructionScript)

(fn FireMultishot
  (bind _projcount (Variables|Default|GetProjCount))
  (bind _arrow (Variables|Default|GetArrow))
  (bind _returnvalue (Math|Conversions|ToFloat(Integer) _projcount))
  (bind _returnvalue_2 (/ 9e+01 _returnvalue))
  ;[0.8021 0.8021 0.8021 0.5] Calculate Inital Angle and Delta Angle for a given number of projectiles
  (LocalVariables|SetInitialAngle (/ (- 9e+01 _returnvalue_2) -2.0))
  (LocalVariables|SetDeltaAngle _returnvalue_2)
  ;[1 0 0 0.5] Loop over each projectile
  (for _index (range 0 (- (Variables|Default|GetProjCount) 1))
    (Game|SpawnActorfromClass "/Game/Upgrades/Testing/BP_Test_Projectile_Arrow.BP_Test_Projectile_Arrow_C" (Math|Transform|MakeTransform (Transformation|GetWorldLocation _arrow) (Math|Rotator|MakeRotator 0.0 0.0 (+ (* _index (LocalVariables|GetDeltaAngle)) (LocalVariables|GetInitialAngle) (.yaw (Transformation|GetWorldRotation _arrow)))) "1.000000,1.000000,1.000000") "Undefined" "MultiplyWithRoot" 0 0)))