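; Test Blueprint that exercises the upgrade manager and game stat systems through on-screen debug prints.
; On BeginPlay it adds an AC_UpgradeManager, removes three entries from the pool, generates upgrades and prints the three resulting options.
; DebugPrintGameStats formats nine stat fields into one printed line.
; Unconnected leftover chains test gold, stat upgrades and mod stats on BP_MainGameInstance but never run.
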(event EventBeginPlay
  (bind _returnvalue (Game|AddComponentbyClass "/Game/Upgrades/AC_UpgradeManager.AC_UpgradeManager_C"))
  (bind _output_get (Variables|Default|SetUpgradeManager _returnvalue))
  (Class|BPIUpgrades|RemovefromPool(Message) _output_get "NewEnumerator0")
  (Class|BPIUpgrades|RemovefromPool(Message) _output_get "NewEnumerator3")
  (Class|BPIUpgrades|RemovefromPool(Message) _output_get "NewEnumerator4")
  (Default|GenerateUpgrades _output_get)
  (bind _upgrade (Default|GetUpgradeOption _output_get))
  (bind _upgrade_2 (Default|GetUpgradeOption _output_get 1))
  (bind _upgrade_3 (Default|GetUpgradeOption _output_get 2))
  (Development|PrintString (Utilities|String|Append (Utilities|String|EnumtoString _upgrade) ", " (Utilities|String|EnumtoString _upgrade_2) ", " (Utilities|String|EnumtoString _upgrade_3)) true true "(R=0.000000,G=0.660000,B=1.000000,A=1.000000)" 5.0))

(event EventTick
  (params (DeltaSeconds :type Float%20%28single-precision%29)))

(fn ConstructionScript)

(fn DebugPrintGameStats
  (params (GameStats :type F%20Game%20Stats%20Structure))
  (LocalVariables|SetStats GameStats)
  (for _index (range 0 8)
    (LocalVariables|SetOutputText (Utilities|String|Append (LocalVariables|GetOutputText) "Stat " (Utilities|String|ToString(Integer) _index) ": " (Utilities|String|ToString(Float) (Utilities|Select :Index _index :Option%200 (.attackdmg (LocalVariables|GetStats)) :Option%201 (.attackspeed (LocalVariables|GetStats)) :Option%202 (.defense (LocalVariables|GetStats)) :Option%203 (.healthregen (LocalVariables|GetStats)) :Option%204 (.healthmax (LocalVariables|GetStats)) :Option%205 (.critrate (LocalVariables|GetStats)) :Option%206 (.critdmg (LocalVariables|GetStats)) :Option%207 (.speed (LocalVariables|GetStats)) :Option%208 (.dashregen (LocalVariables|GetStats)))) " |")))
  (Development|PrintString (LocalVariables|GetOutputText) true true "(R=0.000000,G=0.660000,B=1.000000,A=1.000000)" 2e+01 ""))