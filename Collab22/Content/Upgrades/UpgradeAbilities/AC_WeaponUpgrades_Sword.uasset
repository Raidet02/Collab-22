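; Sword weapon upgrade component that holds and raises the sword's attack stats.
; Three upgrade events add fixed increments to attack size, bleed damage and final strike damage, each exposed through a getter.
; The WeaponAttack event is empty, and its deprecated sphere-trace damage logic remains disconnected, as does the old looking-direction lookup.
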(event EventBeginPlay
  ;[0.15 0.15 0.15 0.5] Delete looking direction
  (|CallParentFunction))

(event EventUpgrade1
  (params (Amount :type Float%20%28double-precision%29))
  ;[1 1 1 0.5] Weapon Attack Size
  (Variables|Default|SetAttackSize (+ 1e+01 (Variables|Default|GetAttackSize))))

(event EventUpgrade2
  (params (Amount :type Float%20%28double-precision%29))
  ;[1 0 0 0.5] Bleed Damage
  (Variables|Default|SetBleedDamage (+ (Variables|Default|GetBleedDamage) 3.0)))

(event EventUpgrade3
  (params (Amount :type Float%20%28double-precision%29))
  ;[1 0 0 0.5] Final Strike Damage
  (Variables|Default|SetFinalStrikeDamage (+ 5.0 (Variables|Default|GetFinalStrikeDamage))))

(event EventWeaponAttack
  (params (Damage :type Float%20%28double-precision%29) (AttackIndex :type Integer))
  ;[0.5 0.5 0.5 0.5] (Depreciated) Single Trace Sphere Attack
)

(fn GetAttackSize
  (return (Variables|Default|GetAttackSize)))

(fn GetBleedDmg
  (return (Variables|Default|GetBleedDamage)))

(fn GetFinalStrikeDmg
  (return (Variables|Default|GetFinalStrikeDamage)))