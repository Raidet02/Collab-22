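; AC_Multishot is an upgrade ability component on the player character that fires a fan of BP_Test_Projectile_Arrow projectiles.
; Attack spawns arrows at the player's LookingDirection, evenly spaced in yaw and centered within a 90-degree arc.
; The first upgrade level sets projectile count and spacing.
; The other two set pierce count and storm chance, but Attack uses neither, and storm chance always evaluates to zero.
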(event EventBeginPlay
  (CallFunction|SetUpgrade1)
  (CallFunction|SetUpgrade2)
  (CallFunction|SetUpgrade3)
  (bind _asbp_player_character (Utilities|Casting|CastToBP_PlayerCharacter (Components|GetOwner)))
  (Variables|Default|SetLooking%20Direction (Variables|/Game/Player/BP_PlayerCharacter.BP_PlayerCharacter_C|GetLookingDirection _asbp_player_character)))

(event EventTick
  (params (DeltaSeconds :type Float%20%28single-precision%29)))

(event EventSetUpgrade1
  (params (Level :type Integer))
  ;[0.8021 0.8021 0.8021 0.5] Initialise multishot variables
  (Variables|Default|SetProjCount (+ Level 1))
  (Variables|Default|SetInitialAngle (/ (- 9e+01 (/ 9e+01 (Math|Conversions|ToFloat(Integer) (Variables|Default|GetProjCount)))) -2.0))
  (Variables|Default|SetDeltaAngle (/ 9e+01 (Math|Conversions|ToFloat(Integer) (Variables|Default|GetProjCount)))))

(event EventSetUpgrade2
  (params (Level :type Integer))
  (Variables|Default|SetPierceCount Level))

(event EventSetUpgrade3
  (params (Level :type Integer))
  (Variables|Default|SetStormChance (* Level 0.0)))

(event EventAttack
  (bind _looking_direction (Variables|Default|GetLooking%20Direction))
  ;[1 0 0 0.5] Fire each projectile
  (for _index (range 0 (- (Variables|Default|GetProjCount) 1))
    (Game|SpawnActorfromClass "/Game/Upgrades/Testing/BP_Test_Projectile_Arrow.BP_Test_Projectile_Arrow_C" (Math|Transform|MakeTransform (Transformation|GetWorldLocation _looking_direction) (Math|Rotator|MakeRotator 0.0 0.0 (+ (* _index (Variables|Default|GetDeltaAngle)) (Variables|Default|GetInitialAngle) (.yaw (Transformation|GetWorldRotation _looking_direction)))) "1.000000,1.000000,1.000000") "Undefined" "MultiplyWithRoot" 0 0)))