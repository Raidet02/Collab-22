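; Bow weapon upgrade component that fires arrow projectiles from the player's looking direction on normal and heavy attacks.
; Three upgrades add multishot, piercing, and arrow storm chance with extra storm damage.
; Both attacks set damage, boosted for later attack indices and for heavy hits, then share one spawn loop.
; The loop fans arrows across an arc centered on the aim yaw, passing pierce and storm stats to each.
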(event Custom|HeavyAttack
  (params (IndexAttack :type Integer) (Dmg :type Float%20%28double-precision%29))
  (bind _returnvalue (* Dmg 1.15))
  (bind _looking_direction (Variables|Default|GetLooking%20Direction))
  ;[1 0 0 0.5] Fire each projectile
  (Utilities|Map|Add (Variables|Default|GetDamageTypeMap) "NewEnumerator0" (Math|Float|SelectFloat (* _returnvalue 1.25) _returnvalue (> IndexAttack 2)))
  (for _index (range 0 (- (Variables|Multishot|GetProjCount) 1))
    (Game|SpawnActorfromClass "/Game/Player/Weapons/Projectiles/BP_Projectile_Bow.BP_Projectile_Bow_C" (Math|Transform|MakeTransform (Transformation|GetWorldLocation _looking_direction) (Math|Rotator|MakeRotator 0.0 0.0 (+ (* _index (Variables|Multishot|GetDeltaAngle)) (Variables|Multishot|GetInitialAngle) (.yaw (Transformation|GetWorldRotation _looking_direction)))) "1.000000,1.000000,1.000000") "Undefined" "MultiplyWithRoot" 0 (Variables|Default|GetPierceCount) (Variables|Default|GetStormChance) (Variables|Default|GetDamageTypeMap) (Variables|Default|GetDamageArrowStorm) 0)))

(event EventBeginPlay
  (|CallParentFunction)
  (bind _playerref (Class|BPIPlayer|GetPlayerRef(Message) (Game|Player|GetPlayerPawn 0)))
  (Variables|Default|SetLooking%20Direction (Variables|/Game/Player/BP_PlayerCharacter.BP_PlayerCharacter_C|GetLookingDirection _playerref)))

(event EventUpgrade3
  (params (Amount :type Float%20%28double-precision%29))
  (bind _damagearrowstorm (Variables|Default|GetDamageArrowStorm))
  (Variables|Default|SetStormChance (+ (Variables|Default|GetStormChance) 5))
  (Utilities|Map|Add _damagearrowstorm "NewEnumerator0" (+ (.Value (Utilities|Map|Find _damagearrowstorm "NewEnumerator0")) 3.0)))

(event EventUpgrade1
  (params (Amount :type Float%20%28double-precision%29))
  ;[0.8021 0.8021 0.8021 0.5] Initialise multishot variables
  (Variables|Multishot|SetProjCount (+ (Variables|Multishot|GetProjCount) 1))
  (Variables|Multishot|SetInitialAngle (/ (- 4e+01 (/ 4e+01 (Math|Conversions|ToFloat(Integer) (Variables|Multishot|GetProjCount)))) -2.0))
  (Variables|Multishot|SetDeltaAngle (/ 4e+01 (Math|Conversions|ToFloat(Integer) (Variables|Multishot|GetProjCount)))))

(event EventUpgrade2
  (params (Amount :type Float%20%28double-precision%29))
  (Variables|Default|SetPierceCount (+ (Variables|Default|GetPierceCount) 1)))

(event EventWeaponAttack
  (params (Damage :type Float%20%28double-precision%29) (AttackIndex :type Integer))
  (bind _looking_direction (Variables|Default|GetLooking%20Direction))
  ;[1 0 0 0.5] Fire each projectile
  (Utilities|Map|Add (Variables|Default|GetDamageTypeMap) "NewEnumerator0" (Math|Float|SelectFloat (* Damage 1.2) Damage (> AttackIndex 2)))
  (for _index (range 0 (- (Variables|Multishot|GetProjCount) 1))
    (Game|SpawnActorfromClass "/Game/Player/Weapons/Projectiles/BP_Projectile_Bow.BP_Projectile_Bow_C" (Math|Transform|MakeTransform (Transformation|GetWorldLocation _looking_direction) (Math|Rotator|MakeRotator 0.0 0.0 (+ (* _index (Variables|Multishot|GetDeltaAngle)) (Variables|Multishot|GetInitialAngle) (.yaw (Transformation|GetWorldRotation _looking_direction)))) "1.000000,1.000000,1.000000") "Undefined" "MultiplyWithRoot" 0 (Variables|Default|GetPierceCount) (Variables|Default|GetStormChance) (Variables|Default|GetDamageTypeMap) (Variables|Default|GetDamageArrowStorm) 0)))