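; Actor component that applies a burn damage-over-time effect to its owning actor, as an upgrade ability effect.
; On BeginPlay it starts a looping timer and spawns the NS_Bleed_Effect Niagara system.
; Each timer tick applies fixed damage to the owner and decrements an Iterations counter.
; When the counter runs out, it clears the timer and destroys both the particle system and itself.
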(event Custom|Event_Damage_Owner
  (if (> (Variables|Default|GetIterations) 0)
    (Game|Damage|ApplyDamage (Components|GetOwner) 4.0 0 0)
    (Variables|Default|SetIterations (- (Variables|Default|GetIterations) 1))
    (else
      (Utilities|Time|ClearandInvalidateTimerbyHandle (Variables|Default|GetTimer))
      (Components|DestroyComponent (Variables|Default|GetParticelSys))
      (Components|DestroyComponent))))

(event EventBeginPlay
  (bind _returnvalue (Utilities|Time|SetTimerbyEvent (delegate Custom|Event_Damage_Owner) 0.5 true))
  (Variables|Default|SetTimer _returnvalue)
  (bind _returnvalue_2 (Niagara|SpawnSystemAttached "/Game/Player/VFX/NS_Bleed_Effect.NS_Bleed_Effect" 0 "None" "0, 0, 0" "0, 0, 0" "KeepRelativeOffset" false))
  (Variables|Default|SetParticelSys _returnvalue_2))

(event EventTick
  (params (DeltaSeconds :type Float%20%28single-precision%29)))