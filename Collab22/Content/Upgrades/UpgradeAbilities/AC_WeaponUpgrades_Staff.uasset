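; Staff weapon upgrade component that scales the staff's effects by upgrade level and fires its projectile.
; Three upgrade events set burn damage, stun duration and corrosion damage as linear multiples of level.
; WeaponAttack spawns BP_Projectile_Staff at LookingDirection, using only its yaw, and passes in DamageTypeMap.
; The upgrade values are not written into that map here, and a note marks this as a pending change.
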(event EventBeginPlay
  (|CallParentFunction) ; This node is disabled and will not be called.\nDrag off pins to build functionality.
)

(event EventTick
  (params (DeltaSeconds :type Float%20%28single-precision%29))
  (|CallParentFunction DeltaSeconds) ; This node is disabled and will not be called.\nDrag off pins to build functionality.
)

(event EventSetUpgrade1
  (params (Level :type Integer))
  ;[0.15 0.15 0.15 0.5] Change For Damage Type Map
  (Variables|Default|SetBurnDamage (* Level 3)))

(event EventSetUpgrade2
  (params (Level :type Integer))
  ;[0.15 0.15 0.15 0.5] Change For Damage Type Map
  (Variables|Default|SetStunDuration (* Level 0.2)))

(event EventSetUpgrade3
  (params (Level :type Integer))
  ;[0.15 0.15 0.15 0.5] Change For Damage Type Map
  (Variables|Default|SetCorrosionDamage (* Level 3)))

(event EventWeaponAttack
  (params (Damage :type Float%20%28double-precision%29))
  (bind _looking_direction (Variables|Default|GetLooking%20Direction))
  (Game|SpawnActorfromClass "/Game/Player/Weapons/Projectiles/BP_Projectile_Staff.BP_Projectile_Staff_C" (Math|Transform|MakeTransform (Transformation|GetWorldLocation _looking_direction) (Math|Rotator|MakeRotator 0.0 0.0 (.yaw (Transformation|GetWorldRotation _looking_direction))) "1.000000,1.000000,1.000000") "Undefined" "MultiplyWithRoot" 0 (Variables|Default|GetDamage%20Type%20Map) 0))