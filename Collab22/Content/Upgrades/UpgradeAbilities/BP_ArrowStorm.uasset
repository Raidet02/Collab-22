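; BP_ArrowStorm is an area damage actor for the Arrow Storm upgrade ability.
; On BeginPlay it starts a looping timer that deals fixed damage to every actor overlapping its sphere collision and counts down an iteration counter.
; When the counter runs out, it clears the timer and destroys itself.
; Each timer tick also prints a debug "Damage" message.
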(event Custom|Event_DamageArea
  (Development|PrintText "Damage" true true "(R=0.000000,G=0.660000,B=1.000000,A=1.000000)" 1.2)
  (if (> (Variables|Default|GetIteration) 0)
    (for _array_element (Collision|GetOverlappingActors (Variables|Default|GetSphereCollision) 0 :!class /Script/Engine.PrimitiveComponent)
      (Game|Damage|ApplyDamage _array_element 6.0 0 0))
    (Variables|Default|SetIteration (- (Variables|Default|GetIteration) 1))
    (else
      (Utilities|Time|ClearandInvalidateTimerbyHandle (Variables|Default|GetTimer))
      (Actor|DestroyActor))))

(event EventBeginPlay
  (bind _returnvalue (Utilities|Time|SetTimerbyEvent (delegate Custom|Event_DamageArea) 1.0 true false 0.1))
  (Variables|Default|SetTimer _returnvalue))

(event Collision|EventActorBeginOverlap
  (params (OtherActor :type Actor%20Object%20Reference)))

(event EventTick
  (params (DeltaSeconds :type Float%20%28single-precision%29)))

(fn ConstructionScript)