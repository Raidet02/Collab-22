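; BP_MetaUpgrades handles meta-progression purchases for Attack, Defence and Attack Speed stat upgrades.
; MetaUpgradeEvent passes a stat type to UpgradeStat, which checks a placeholder currency against that stat's cost and deducts it when affordable.
; Each purchase compounds that stat's modifier and cost by fixed multipliers in the StatMod and StatCost structs, then returns whether it succeeded.
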(event Custom|MetaUpgradeEvent
  (params (StatType :type E_StatType%20Enum :default "NewEnumerator0"))
  (CallFunction|UpgradeStat StatType))

(fn UpgradeStat
  (params (Stat :type E_StatType%20Enum :default "NewEnumerator0"))
  (LocalVariables|SetCurrentStat Stat)
  (bind _output_get (LocalVariables|SetValid (>= (- (Variables|Default|GetCurrency%28Placeholder%29) (Utilities|Select :Index (LocalVariables|GetCurrentStat) :NewEnumerator0 (.attack (Variables|Default|GetStatCost)) :NewEnumerator1 (.defence (Variables|Default|GetStatCost)) :NewEnumerator2 (.attackspeed (Variables|Default|GetStatCost)))) 0.0)))
  (if _output_get
    (Variables|Default|SetCurrency%28Placeholder%29 (- (Variables|Default|GetCurrency%28Placeholder%29) (Utilities|Select :Index (LocalVariables|GetCurrentStat) :NewEnumerator0 (.attack (Variables|Default|GetStatCost)) :NewEnumerator1 (.defence (Variables|Default|GetStatCost)) :NewEnumerator2 (.attackspeed (Variables|Default|GetStatCost)))))
    ;[0.15 0.15 0.15 0.5] Updating stats and upgrade costs
    (switch Utilities|FlowControl|Switch|SwitchonE_StatType (LocalVariables|GetCurrentStat)
      (:NewEnumerator0
        (Variables|Default|SetStatMod (Utilities|Struct|MakeF_UpgradeStats (* (.attack (Variables|Default|GetStatMod)) 1.1) (.defence (Variables|Default|GetStatMod)) (.attackspeed (Variables|Default|GetStatMod))))
        (Variables|Default|SetStatCost (Utilities|Struct|MakeF_UpgradeStats (* (.attack (Variables|Default|GetStatCost)) 1.5) (.defence (Variables|Default|GetStatCost)) (.attackspeed (Variables|Default|GetStatCost)))))
      (:NewEnumerator1
        (Variables|Default|SetStatMod (Utilities|Struct|MakeF_UpgradeStats (.attack (Variables|Default|GetStatMod)) (* (.defence (Variables|Default|GetStatMod)) 1.1) (.attackspeed (Variables|Default|GetStatMod))))
        (Variables|Default|SetStatCost (Utilities|Struct|MakeF_UpgradeStats (.attack (Variables|Default|GetStatCost)) (* (.defence (Variables|Default|GetStatCost)) 1.5) (.attackspeed (Variables|Default|GetStatCost)))))
      (:NewEnumerator2
        (Variables|Default|SetStatMod (Utilities|Struct|MakeF_UpgradeStats (.attack (Variables|Default|GetStatMod)) (.defence (Variables|Default|GetStatMod)) (* (.attackspeed (Variables|Default|GetStatMod)) 1.1)))
        (Variables|Default|SetStatCost (Utilities|Struct|MakeF_UpgradeStats (.attack (Variables|Default|GetStatCost)) (.defence (Variables|Default|GetStatCost)) (* (.attackspeed (Variables|Default|GetStatCost)) 1.5))))))
  (return (LocalVariables|GetValid)))