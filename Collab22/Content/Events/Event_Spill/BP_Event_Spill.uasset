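; Timed spill hazard event that moves to the player's location on BeginPlay (a testing placement) and destroys itself after EventLength.
; Box overlap cuts the speed stat through stats message calls and starts a looping damage timer.
; End overlap writes back the overlapped component's current speed without clearing the timer.
; OverlapDamageAndSlow bundles damage and speed halving, but the event graph never calls it.
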(event OnComponentBeginOverlap(Box)
  (params (OverlappedComponent :type Primitive%20Component%20Object%20Reference) (OtherActor :type Actor%20Object%20Reference) (OtherComp :type Primitive%20Component%20Object%20Reference) (OtherBodyIndex :type Integer) (bFromSweep :type Boolean) (SweepResult :type Hit%20Result%20Structure%20%28by%20ref%29))
  (bind _currentstats (Class|BPIUpgrades|GetCurrentGameStats(Message) OverlappedComponent))
  (Class|BPIControllerVars|UpdateGameStats(Message) OtherActor (Utilities|Struct|MakeF_GameStats 1.0 1.0 1.0 0.0 1.0 1.0 1.0 (/ (.speed _currentstats) 1e+07) 1.0) "NewEnumerator7")
  (Development|PrintString (Utilities|String|ToString(Float) (/ (.speed _currentstats) 1e+07)))
  (Utilities|Time|SetTimerbyEvent (delegate Custom|DOT) (Variables|Default|GetDOTTimer) true))

(event OnComponentEndOverlap(Box)
  (params (OverlappedComponent :type Primitive%20Component%20Object%20Reference) (OtherActor :type Actor%20Object%20Reference) (OtherComp :type Primitive%20Component%20Object%20Reference) (OtherBodyIndex :type Integer))
  (bind _currentstats (Class|BPIUpgrades|GetCurrentGameStats(Message) OverlappedComponent))
  (Class|BPIControllerVars|UpdateGameStats(Message) OverlappedComponent (Utilities|Struct|MakeF_GameStats 1.0 1.0 1.0 0.0 1.0 1.0 1.0 (.speed _currentstats) 1.0) "NewEnumerator7")
  (Development|PrintString (Utilities|String|ToString(Float) (.speed _currentstats))))

(event Custom|EndEvent
  ;[0.15 0.15 0.15 0.5] Spawns the actor then deletes it, currently spawns on player for testing but swap that out for proper location once it is decided
  (Development|PrintString "Spill Over")
  (Actor|DestroyActor))

(event Custom|DOT
  (Game|Damage|ApplyDamage (stale OnComponentBeginOverlap(Box) OtherActor) 1.0 0 0))

(event EventBeginPlay
  ;[0.15 0.15 0.15 0.5] Spawns the actor then deletes it, currently spawns on player for testing but swap that out for proper location once it is decided
  (Transformation|SetActorLocation (Transformation|GetActorLocation (Variables|Default|GetPlayerRef)) false false)
  (Utilities|Time|SetTimerbyEvent (delegate Custom|EndEvent) (Variables|Default|GetEventLength)))

(fn ConstructionScript
  (|CallParentFunction))

(fn OverlapDamageandSlow
  (params (ActorRef :type Actor%20Object%20Reference))
  (Game|Damage|ApplyDamage ActorRef 1.0 0 0)
  ;[0.15 0.15 0.15 0.5] Updates the player speed for when in the spill
  (bind _currentstats (Class|BPIUpgrades|GetCurrentGameStats(Message) ActorRef))
  (Class|BPIControllerVars|UpdateGameStats(Message) ActorRef (Utilities|Struct|MakeF_GameStats 1.0 1.0 1.0 0.0 1.0 1.0 1.0 (/ (.speed _currentstats) 2.0) 1.0) "NewEnumerator7"))