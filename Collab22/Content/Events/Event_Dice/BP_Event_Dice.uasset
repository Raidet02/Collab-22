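; Dice event actor that plays a throw cinematic and rolls a physics die to randomly boost attack for the player or enemies.
; BeginPlay gathers enemies, starts the level sequence, then launches the die with impulse and random torque.
; A timer stops it, and the highest mesh socket maps to the rolled side before the actor self-destructs.
; Rolls above nine favor the player, others enemies; timed buff removal is marked unfinished.
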(event Custom|Rolled
  ;[0.15 0.15 0.15 0.5] If the die has been rolled it will check if it is slow or not moving before firing the read value event then set rolled side for the buffs to be called
  (if (<= (Math|Vector|VectorLength (Transformation|GetComponentVelocity (Variables|Default|GetSkeletalMesh))) 0.0)
    (Utilities|FlowControl|DoOnce false
      (:Completed
        (bind _siderolled (CallFunction|ReadValue))
        (Variables|Default|SetRolledSide (.Value (Utilities|Map|Find (Variables|Default|GetSideValues) _siderolled)))
        (Utilities|FlowControl|Delay 5.0)
        (Actor|DestroyActor)))))

(event Custom|EndBuffs
  (bind _playerref (Variables|Default|GetPlayerRef))
  (bind _currentgamestats (Variables|/Game/Player/BP_PlayerCharacter.BP_PlayerCharacter_C|GetCurrentGameStats _playerref))
  (bind (_attackdmg _attackspeed _defense _healthregen _healthmax _critrate _critdmg _speed _dashregen) (Utilities|Struct|BreakF_GameStats _currentgamestats))
  (if (> (Variables|Default|GetRolledSide) 9)
    (Class|BPIControllerVars|UpdateGameStats(Message) (Variables|Default|GetPlayerRef) (Utilities|Struct|MakeF_GameStats (/ _attackdmg 1.5) _attackspeed _defense _healthregen _healthmax _critrate _critdmg _speed _dashregen) "NewEnumerator0")
    (else
      (for _array_element (Variables|Default|GetEnemyRefArray)
        (Class|BPIEnemy|NerfEnemyAttack(Message) _array_element)))))

(event Custom|FinisRoll
  ;[0.15 0.15 0.15 0.5] Stop the roll
  (Class|PrimitiveComponent|SetAllPhysicsLinearVelocity (Variables|Default|GetSkeletalMesh) "0, 0, 0" false)
  (CallFunction|Rolled)
  (CallFunction|Buffs))

(event EventBeginPlay
  ;[0.15 0.15 0.15 0.5] Plays Cinematic
  (|CallParentFunction)
  (bind _outactors (Actor|GetAllActorsOfClass "/Game/Enemies/BP_Enemy_Parent.BP_Enemy_Parent_C"))
  (for _array_element _outactors
    (Utilities|Array|AddUnique (Variables|Default|GetEnemyRefArray) _array_element))
  (Class|BPIPlayer|CinimaticRelocation(Message) (Variables|Default|GetPlayerRef))
  (Class|PlayerController|SetCinematicMode (Game|GetPlayerController 0) true false true false false)
  (bind _returnvalue (Game|SpawnActorfromClass :Class "/Game/Cinematics/LSA_EventDiceRoll.LSA_EventDiceRoll_C" :SpawnTransform (Math|Transform|MakeTransform (Transformation|GetWorldLocation (Variables|Default|GetDefaultSceneRoot)) "0, 0, 0" "1.000000,1.000000,1.000000") :CollisionHandlingOverride "Undefined" :TransformScaleMethod "MultiplyWithRoot" :LevelSequenceAsset "/Game/Cinematics/LS_EventDiceRoll.LS_EventDiceRoll" :Instigator 0))
  ;[0.15 0.15 0.15 0.5] Throw the die
  (Sequencer|Player|Play (Variables|/Script/LevelSequence.LevelSequenceActor|GetSequencePlayer _returnvalue) :!class /Script/MovieScene.MovieSceneSequencePlayer)
  (Utilities|FlowControl|Delay 5.0)
  (CallFunction|RollDie (Variables|DiceThrow|GetThrow%20Power) (Variables|DiceThrow|GetRotate%20Power)))

(fn ConstructionScript
  (|CallParentFunction))

(fn RollDie
  (params (ThrowPower :type Float%20%28single-precision%29) (RotatePower :type Float%20%28single-precision%29))
  (bind _skeletalmesh (Variables|Default|GetSkeletalMesh))
  (bind _returnvalue (Physics|GetMass _skeletalmesh))
  (bind _returnvalue_2 (* "-1.000000,0.000000,0.000000" _returnvalue ThrowPower))
  (bind (_x _y _z) (Math|Vector|BreakVector _returnvalue_2))
  ;[0.15 0.15 0.15 0.5] Throw direction and strength
  (Transformation|SetWorldLocation (Variables|Default|GetSkeletalMesh) "40.000000,40.000000,900.000000" false true)
  (Physics|AddImpulse (Variables|Default|GetSkeletalMesh) (Math|Vector|MakeVector _x _y (Math|Float|Absolute(Float) _z)) "None" false)
  ;[0.15 0.15 0.15 0.5] Dice rotation
  (Class|PrimitiveComponent|AddTorqueinDegrees (Variables|Default|GetSkeletalMesh) (* RotatePower (Physics|GetMass (Variables|Default|GetSkeletalMesh)) (Math|Random|RandomUnitVector) ThrowPower) "None" false)
  (bind _returnvalue_3 (Utilities|Time|SetTimerbyEvent (EventDispatchers|CreateEvent :!event Custom|FinisRoll) (Variables|Timer|GetDiceStopTime)))
  (Variables|Default|SetFinishRollTimer _returnvalue_3))

(fn ReadValue
  ;[0.15 0.15 0.15 0.5] Loops through sockets to see which one is higher then sets that to the highest value and retuns the name
  (for _array_element (Transformation|GetAllSocketNames (Variables|Default|GetSkeletalMesh))
    (if (> (.z (Transformation|GetSocketLocation (Variables|Default|GetSkeletalMesh) _array_element)) (LocalVariables|GetL_HighestValue))
      (LocalVariables|SetL_HighestValue (.z (Transformation|GetSocketLocation (Variables|Default|GetSkeletalMesh) _array_element)))
      (LocalVariables|SetL_HighestName _array_element)))
  (return (LocalVariables|GetL_HighestName)))

(fn Buffs
  (bind _playerref (Variables|Default|GetPlayerRef))
  (bind _currentgamestats (Variables|/Game/Player/BP_PlayerCharacter.BP_PlayerCharacter_C|GetCurrentGameStats _playerref))
  (bind (_attackdmg _attackspeed _defense _healthregen _healthmax _critrate _critdmg _speed _dashregen) (Utilities|Struct|BreakF_GameStats _currentgamestats))
  ;[0.15 0.15 0.15 0.5] Checks if rolled side is more than 9 then gets ready to buff the player or the enemy
  (if (> (Variables|Default|GetRolledSide) 9)
    (Class|BPIControllerVars|UpdateGameStats(Message) (Variables|Default|GetPlayerRef) (Utilities|Struct|MakeF_GameStats (* _attackdmg 1.5) _attackspeed _defense _healthregen _healthmax _critrate _critdmg _speed _dashregen) "NewEnumerator0")
    (else
      (for _array_element (Variables|Default|GetEnemyRefArray)
        (Class|BPIEnemy|BuffEnemyAttack(Message) _array_element))))
  ;[0.15 0.15 0.15 0.5] Timer to end Buff  with event not working how I want, try to figure out without using delay
  (Utilities|Time|SetTimerbyEvent (EventDispatchers|CreateEvent :!event Custom|EndBuffs) (LocalVariables|GetBuffLengthTimer))
  ;[0.15 0.15 0.15 0.5] Replace with end buff code when ready
  (Development|PrintString "End Buffs"))