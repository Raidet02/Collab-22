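; BP_Event_DmScreen is an event actor that makes screens appear at the player's position for a limited time.
; On BeginPlay it places its root below the player referenced by PlayerRef, then raises it to the player's location with a short MoveComponentTo.
; It also starts a ten-second timer, apparently bound to DestroyScreens, which destroys the actor.
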(event Custom|Destroy%20Screens
  ;[0.15 0.15 0.15 0.5] Destroys the screens
  (Actor|DestroyActor))

(event EventBeginPlay
  (bind _playerref (Variables|Default|GetPlayerRef))
  (bind _returnvalue (Transformation|GetActorLocation _playerref))
  ;[0.15 0.15 0.15 0.5] Spawns the screens on the player position
  (|CallParentFunction)
  (Transformation|SetWorldLocation (Variables|Default|GetDefaultSceneRoot) (Math|Vector|MakeVector (.x _returnvalue) (.y _returnvalue) (- (.z _returnvalue) 2e+02)) false false)
  (Components|MoveComponentTo (Variables|Default|GetDefaultSceneRoot) (Transformation|GetActorLocation (Variables|Default|GetPlayerRef)) "0, 0, 0" false false 2.0 false)
  (Utilities|Time|SetTimerbyEvent (EventDispatchers|CreateEvent :!event Custom|Destroy%20Screens) 1e+01))

(fn ConstructionScript
  (|CallParentFunction))