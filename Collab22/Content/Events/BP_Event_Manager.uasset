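; BP_Event_Manager is an actor that periodically triggers random game events from an array of event classes.
; Once started, a looping timer picks a random entry and broadcasts it through the OnEventChosen dispatcher with its spawn delay.
; A second timer then spawns that class at the manager's location and removes it from the array so it is not picked again.
; GetCurrentEvent exposes the latest chosen event.
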(event Custom|PickEventTimer
  (bind _eventarray (Variables|Default|GetEventArray))
  (bind _eventspawntime (Variables|Default|GetEventSpawnTime))
  ;[0.15 0.15 0.15 0.5] Spawn a random event in an array
  (bind _output_get (Variables|Default|SetEventIndex (Math|Random|RandomIntegerinRange 0 (- (Utilities|Array|Length _eventarray) 1))))
  (bind _output_get_2 (Variables|Default|SetChosenEvent (Utilities|Array|Get(acopy) _eventarray _output_get)))
  (Default|CallOnEventChosen _output_get_2 _eventspawntime)
  (Utilities|Time|SetTimerbyEvent (delegate Custom|SpawnEvent) _eventspawntime))

(event Custom|SpawnEvent
  (bind _eventarray (Variables|Default|GetEventArray))
  ;[0.15 0.15 0.15 0.5] Spawn a random event in an array
  (bind _returnvalue (Game|SpawnActorfromClass (Utilities|Array|Get(acopy) _eventarray (stale Custom|PickEventTimer _output_get)) (Math|Conversions|ToTransform(Vector) (Transformation|GetWorldLocation (Variables|Default|GetDefaultSceneRoot))) "Undefined" "MultiplyWithRoot" 0 0))
  (Variables|Default|SetSpawnedEvent _returnvalue)
  (Utilities|Array|RemoveIndex _eventarray (stale Custom|PickEventTimer _output_get)))

(event EventStartEventManager
  (Utilities|Time|SetTimerbyEvent (delegate Custom|PickEventTimer) 145.0 true))

(fn ConstructionScript)

(fn GetCurrentEvent
  (return (Variables|Default|GetChosenEvent)))